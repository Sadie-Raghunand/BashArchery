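; Player actor for a turn-based archery minigame, playable by flex controller or keyboard, with a practice mode that grants near-infinite arrows.
; Registers with the turn manager and takes a target, then fires arrows with hold-time or flex-based force, re-randomizing wind each shot.
; Off-turn players' shots add to the wind instead.
; Tick line-traces three wind-adjusted landing indicators; keyboard yaw also turns the capture camera, while controller rotation is hard-disabled.
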(event Input|EnhancedActionEvents|EnhancedInputActionIA_Movement
  (params (ActionValue :type Vector%202D%20Structure) (ElapsedSeconds :type Float%20%28double-precision%29) (TriggeredSeconds :type Float%20%28double-precision%29) (InputAction :type Input%20Action%20Object%20Reference :default "/MinigameCore/Input/IA_Movement.IA_Movement"))
  ;[1 1 1] Test rotation with arrow keys
  (CallFunction|RotatewithKeyboard ActionValue))

(event Input|EnhancedActionEvents|EnhancedInputActionIA_MediumFlex
  (params (ActionValue :type Boolean) (ElapsedSeconds :type Float%20%28double-precision%29) (TriggeredSeconds :type Float%20%28double-precision%29) (InputAction :type Input%20Action%20Object%20Reference :default "/LimbitlessBluetoothPlugin/InputActions/IA_MediumFlex.IA_MediumFlex"))
  ;[1 1 1 1 12] Use analog flex for strength of arrow launch
  (Development|PrintString "Medium flex ")
  (Variables|Default|SetSelectionSet 1)
  (Utilities|IsValid (Variables|Default|GetThisArrow) ; Check if there is already a arrow in scene to prevent playe from spamming in one direction
    (:Is%20Valid
      (Development|PrintString "Arrow in scene already"))
    (:Is%20Not%20Valid
      (CallFunction|ChangeArrowForce)
      (bind _delaytime (CallFunction|ShootArrow (Variables|Default|GetForceValToPass)))
      (Utilities|FlowControl|Delay _delaytime)
      (Appearance|SetColorandOpacity (Variables|/Game/Blueprints/ArcheryMinigameBlueprints/UI/BP_ArcheryUI.BP_ArcheryUI_C|GetWindValUI (Variables|Default|GetWindUI)) (Utilities|Struct|MakeSlateColor "(R=0.049872,G=0.562500,B=0.000000,A=1.000000)") :!class /Script/UMG.TextBlock))))

(event Input|EnhancedActionEvents|EnhancedInputActionIA_Button1
  (params (ActionValue :type Boolean) (ElapsedSeconds :type Float%20%28double-precision%29) (TriggeredSeconds :type Float%20%28double-precision%29) (InputAction :type Input%20Action%20Object%20Reference :default "/MinigameCore/Input/IA_Button1.IA_Button1"))
  ;[1 1 1 1 12] Keyboard/spacebar for shooting
  (:Ongoing
    (if (< (Variables|Default|GetSecondsHeld) 2.0) ; Check if force is less than 2, is so keep increasing so long as key is held
      (Variables|Default|SetSecondsHeld (+ (Variables|Default|GetSecondsHeld) 0.1))))
  (:Completed
    (Development|PrintString (Utilities|String|ToString(Float) (Variables|Default|GetSecondsHeld)) true true "(R=1.000000,G=0.382696,B=0.000000,A=1.000000)")
    (Utilities|IsValid (Variables|Default|GetThisArrow) ; Check if there is already a arrow in scene to prevent playe from spamming in one direction
      (:Is%20Valid
        (Development|PrintString "Arrow in scene already"))
      (:Is%20Not%20Valid
        (Development|PrintString "No active arrow" true true "(R=0.000000,G=1.000000,B=0.066729,A=1.000000)")
        (bind _delaytime (CallFunction|ShootArrow (Variables|Default|GetSecondsHeld)))
        (Utilities|FlowControl|Delay _delaytime)
        (Default|CallWindUIColorChange)
        (Variables|Default|SetSecondsHeld 0.0)))))

(event Input|EnhancedActionEvents|EnhancedInputActionIA_LightFlex
  (params (ActionValue :type Boolean) (ElapsedSeconds :type Float%20%28double-precision%29) (TriggeredSeconds :type Float%20%28double-precision%29) (InputAction :type Input%20Action%20Object%20Reference :default "/LimbitlessBluetoothPlugin/InputActions/IA_LightFlex.IA_LightFlex"))
  ;[1 1 1 1 12] Use analog flex for strength of arrow launch
  (Development|PrintString "Light flex")
  (Variables|Default|SetSelectionSet 0)
  (Utilities|IsValid (Variables|Default|GetThisArrow) ; Check if there is already a arrow in scene to prevent playe from spamming in one direction
    (:Is%20Valid
      (Development|PrintString "Arrow in scene already"))
    (:Is%20Not%20Valid
      (CallFunction|ChangeArrowForce)
      (bind _delaytime (CallFunction|ShootArrow (Variables|Default|GetForceValToPass)))
      (Utilities|FlowControl|Delay _delaytime)
      (Appearance|SetColorandOpacity (Variables|/Game/Blueprints/ArcheryMinigameBlueprints/UI/BP_ArcheryUI.BP_ArcheryUI_C|GetWindValUI (Variables|Default|GetWindUI)) (Utilities|Struct|MakeSlateColor "(R=0.049872,G=0.562500,B=0.000000,A=1.000000)") :!class /Script/UMG.TextBlock))))

(event Input|EnhancedActionEvents|EnhancedInputActionIA_StrongFlex
  (params (ActionValue :type Boolean) (ElapsedSeconds :type Float%20%28double-precision%29) (TriggeredSeconds :type Float%20%28double-precision%29) (InputAction :type Input%20Action%20Object%20Reference :default "/LimbitlessBluetoothPlugin/InputActions/IA_StrongFlex.IA_StrongFlex"))
  ;[1 1 1 1 12] Use analog flex for strength of arrow launch
  (Development|PrintString "Strong flex")
  (Variables|Default|SetSelectionSet 2)
  (Utilities|IsValid (Variables|Default|GetThisArrow) ; Check if there is already a arrow in scene to prevent playe from spamming in one direction
    (:Is%20Valid
      (Development|PrintString "Arrow in scene already"))
    (:Is%20Not%20Valid
      (CallFunction|ChangeArrowForce)
      (bind _delaytime (CallFunction|ShootArrow (Variables|Default|GetForceValToPass)))
      (Utilities|FlowControl|Delay _delaytime)
      (Appearance|SetColorandOpacity (Variables|/Game/Blueprints/ArcheryMinigameBlueprints/UI/BP_ArcheryUI.BP_ArcheryUI_C|GetWindValUI (Variables|Default|GetWindUI)) (Utilities|Struct|MakeSlateColor "(R=0.049872,G=0.562500,B=0.000000,A=1.000000)") :!class /Script/UMG.TextBlock))))

(event EventBeginPlay
  (CallFunction|InitValues)
  (Transformation|SetActorRotation "0, 0, 0") ; Test w/o controller, get rid of later
  (Utilities|FlowControl|Delay 0.3)
  (CallFunction|RandomizeWindDirection))

(event EventTick
  (params (DeltaSeconds :type Float%20%28single-precision%29))
  (CallFunction|RotatePlayer (Input|EnhancedActionValues|GetIA_Rotation))
  (CallFunction|LinetraceIndicator))

(fn ConstructionScript)

(fn ShootArrow
  (params (ForceOnArrow :type Float%20%28double-precision%29))
  (bind _defaultsceneroot (Variables|Components|GetDefaultSceneRoot))
  (bind _returnvalue (Transformation|GetWorldTransform _defaultsceneroot))
  (bind (_location _rotation _scale) (Math|Transform|BreakTransform _returnvalue))
  (if (Variables|/Game/Blueprints/ArcheryMinigameBlueprints/BP_ATurnManager.BP_ATurnManager_C|GetinCutscene (Variables|Default|GetTurnManager)) ; Check if game is switching player turns and prevent input from occuring
    (if (Variables|/Script/MinigameCore.MinigameBase|GetbIsPractice (Variables|/Game/Blueprints/ArcheryMinigameBlueprints/BP_ATurnManager.BP_ATurnManager_C|GetGameMode (Variables|Default|GetTurnManager))) ; If inCutscene is true but in practice mode, ignore cutscene
      (if (== (Variables|/Game/Blueprints/ArcheryMinigameBlueprints/BP_ATurnManager.BP_ATurnManager_C|GetPlayerTurn (Variables|Default|GetTurnManager)) (Variables|Default|GetThisPlayerNum)) :!label _label ; Prevent input if it is not this player's turn
        _
        (elif (Variables|/Script/MinigameCore.MinigameBase|GetbIsPractice (Variables|/Game/Blueprints/ArcheryMinigameBlueprints/BP_ATurnManager.BP_ATurnManager_C|GetGameMode (Variables|Default|GetTurnManager))) ; If in practice mode, allow all players to shoot\n\nHowever, predicament exists that they cannot all shoot at the\nvisible target
          _
          (else
            (bind _delaytime (CallFunction|PlayersChangeWind ForceOnArrow)) ; If it is not the player's turn, give them the ability to change the wind factor
            (return _delaytime))))
      (if (> (Variables|Default|GetArrows) 0)
        (bind _returnvalue_2 (Game|SpawnActorfromClass "/Game/Blueprints/ArcheryMinigameBlueprints/BP_AArrow.BP_AArrow_C" (Math|Transform|MakeTransform (+ (Transformation|GetActorLocation) "10.000000,0.000000,0.000000") _rotation _scale) "Undefined" "OverrideRootScale" 0 0)) ; Instantiate arrow
        ;[0.15 0.15 0.15 0.5] Testing - Checking spawn location of arrow (front or back of target)
        (if (> (.X (Math|Vector|BreakVector (Transformation|GetActorLocation _returnvalue_2))) (.X (Math|Vector|BreakVector (Transformation|GetWorldLocation (Variables|/Game/Blueprints/ArcheryMinigameBlueprints/BP_ATarget.BP_ATarget_C|GetTargetRing (Utilities|Array|Get(acopy) (Variables|/Game/Blueprints/ArcheryMinigameBlueprints/BP_ATargetParent.BP_ATargetParent_C|GetTargetRings (Variables|Default|GetAssignedTarget)))))))) ; Checking if spawns behind or in front of target
          (Development|PrintString "arrow spawns nbehind target") ; This is whats happening, not good!
          (else
            (Development|PrintString "arrow spawns in front of target")))
        (Variables|/Game/Blueprints/ArcheryMinigameBlueprints/BP_AArrow.BP_AArrow_C|SetPlayer _returnvalue_2 self)
        (bind _output_get (Variables|Default|SetThisArrow _returnvalue_2))
        (Variables|/Game/Blueprints/ArcheryMinigameBlueprints/BP_AArrow.BP_AArrow_C|SetMultiplier _output_get ForceOnArrow) ; Set multiplier to increase play rate on arrow
        (Math|Integer|DecrementInt (Variables|Default|GetArrows)
          (:%20%20
            ;[1 1 1] Wind and player turns
            (CallFunction|RandomizeWindDirection)
            (if (<= (Variables|Default|GetArrows) 0) ; If arrows are out
              (Development|PrintString "Player is out of arrows, true")
              (Default|SetLastArrow (Variables|Default|GetThisArrow))
              (return 0.0)
              (else
                (Development|PrintString "Not out of arrows")
                (Default|CallSetNumArrowsUI (Variables|/Game/Blueprints/ArcheryMinigameBlueprints/BP_ATurnManager.BP_ATurnManager_C|GetGameMode (Variables|Default|GetTurnManager)) (Variables|Default|GetThisPlayerNum) (Variables|Default|GetArrows) (Variables|Default|GetUIColor))))))))
    (else
      (goto _label))))

(fn InitValues
  (bind _returnvalue (Actor|GetActorOfClass "/MinigameCore/Game/BP_MinigameCapture.BP_MinigameCapture_C"))
  (Variables|Default|SetCamera _returnvalue)
  (bind _returnvalue_2 (Actor|GetActorOfClass "/Game/Blueprints/ArcheryMinigameBlueprints/BP_ATurnManager.BP_ATurnManager_C"))
  (bind _output_get (Variables|Default|SetTurnManager _returnvalue_2))
  (bind _firstplayer (CallFunction|CheckifFirstPlayer))
  (if _firstplayer
    (Variables|Default|SetThisPlayerNum 0) ; Will this break w/more than 1 player? Can't test without multiple controllers
    (else
      (Variables|Default|SetThisPlayerNum (Utilities|Array|Length (Variables|/Game/Blueprints/ArcheryMinigameBlueprints/BP_ATurnManager.BP_ATurnManager_C|GetPlayers (Variables|Default|GetTurnManager)))) ; Set which turn this player has, 0-3
    ))
  (Utilities|Array|Add (Variables|/Game/Blueprints/ArcheryMinigameBlueprints/BP_ATurnManager.BP_ATurnManager_C|GetPlayers _output_get) self)
  (Math|Integer|IncrementInt (Variables|/Game/Blueprints/ArcheryMinigameBlueprints/BP_ATurnManager.BP_ATurnManager_C|GetTurnsTotal _output_get)
    (:%20%20
      (Variables|Default|SetAssignedTarget (Utilities|Array|Get(acopy) (Variables|/Game/Blueprints/ArcheryMinigameBlueprints/BP_ATurnManager.BP_ATurnManager_C|GetTargets (Variables|Default|GetTurnManager)) (Variables|Default|GetThisPlayerNum)))
      (bind _asbp_archery_ui (Utilities|Casting|CastToBP_ArcheryUIClass (Variables|/Script/MinigameCore.MinigameBase|GetMinigameUIClass (Variables|/Game/Blueprints/ArcheryMinigameBlueprints/BP_ATurnManager.BP_ATurnManager_C|GetGameMode (Variables|Default|GetTurnManager))))
        (:then
          (bind _returnvalue_3 (Game|ConstructObjectfromClass _asbp_archery_ui))
          (Variables|Default|SetWindUI _returnvalue_3)
          (CallFunction|SetPositionatBegining)
          (if (Variables|/Script/MinigameCore.MinigameBase|GetbIsPractice (Variables|/Game/Blueprints/ArcheryMinigameBlueprints/BP_ATurnManager.BP_ATurnManager_C|GetGameMode (Variables|Default|GetTurnManager))) ; Set realistically infinite number of arrows in practice mode
            (Variables|Default|SetArrows 2147483647)
            (bind _outactors (Actor|GetAllActorswithTag "PracticeTarget"))
            (bind _asbp_atarget_parent (Utilities|Casting|CastToBP_ATargetParent (Utilities|Array|Get(acopy) _outactors)))
            (Variables|Default|SetPracticeTarget _asbp_atarget_parent)))
        (:CastFailed
          (Development|PrintString "wind cast failed"))))))

(fn RotatePlayer
  (params (RotVal :type Vector :default "0.000000,0.000000,1.000000"))
  (bind _z (Math|Vector|BreakVector RotVal))
  (bind _returnvalue (Math|Rotator|MakeRotator 0.0 0.0 _z))
  (if (not true) ; Prevent input between player turn changes
    (bind _inrange (CallFunction|ChangeTotalRotVal (.Yaw (Math|Rotator|BreakRotator _returnvalue))))
    (if _inrange ; Only if rotation is in range does the rotation occur, else do nothing
      (Transformation|AddRelativeRotation (Variables|Components|GetDefaultSceneRoot) _returnvalue false false)
      (Transformation|AddRelativeRotation (Variables|/Script/Engine.Actor|GetRootComponent (Variables|Default|GetCamera)) _returnvalue false false) ; Also move camera to match rotation
      (Transformation|SetActorRotation (Transformation|GetActorRotation (Variables|Default|GetCamera)))
      (else
        (Class|PlayerRotationComponent|ResetInitialOrientation (Variables|Components|GetPlayerRotation)) ; Set to edge of range?
      ))))

(fn RandomizeWindDirection
  (bind _output_get (Variables|Default|SetWind (Math|Random|RandomFloatinRange -1e+01 1e+01)))
  (Default|CallWindUIChange :WindValNum (Math|Conversions|ToFloat(Integer) (Math|Float|Round _output_get))))

(fn PlayersChangeWind
  (params (WindAdditive :type Float%20%28double-precision%29))
  (bind _windui (Variables|Default|GetWindUI))
  (bind _windvalui (Variables|/Game/Blueprints/ArcheryMinigameBlueprints/UI/BP_ArcheryUI.BP_ArcheryUI_C|GetWindValUI _windui))
  (Development|PrintString (Utilities|String|Append "Not this player's turn, player turn is" (Utilities|String|ToString(Integer) (Variables|/Game/Blueprints/ArcheryMinigameBlueprints/BP_ATurnManager.BP_ATurnManager_C|GetPlayerTurn (Variables|Default|GetTurnManager))) ", This is player " (Utilities|String|ToString(Integer) (Variables|Default|GetThisPlayerNum))))
  (bind _output_get (Variables|Default|SetWind (+ (Variables|Default|GetWind) WindAdditive)))
  (Variables|/Script/UMG.TextBlock|SetText _windvalui (Utilities|Text|ToText(Float) _output_get "HalfToEven"))
  (Development|PrintString "Wind changed" true true "(R=1.000000,G=0.292893,B=0.823223,A=1.000000)")
  (Appearance|SetColorandOpacity _windvalui (Utilities|Struct|MakeSlateColor "(R=1.000000,G=0.000000,B=0.006574,A=1.000000)") :!class /Script/UMG.TextBlock)
  (return 1.0))

(fn ChangeTotalRotVal
  (params (ChangeVal :type Float%20%28double-precision%29))
  (if (Math|Float|InRange(Float) (+ ChangeVal (Variables|Default|GetTotalRotation)) -45.0 45.0) ; Check if in of range, do nothing if it isnt
    (Variables|Default|SetTotalRotation (+ ChangeVal (Variables|Default|GetTotalRotation))) ; Change variable value if it remains in range
    (return true) ; Return true, in range
    (else
      (return false) ; Return false, out of range
    )))

(fn SetPositionatBegining
  (Transformation|SetActorLocation (+ (Transformation|GetActorLocation (Utilities|Array|Get(acopy) (Variables|/Game/Blueprints/ArcheryMinigameBlueprints/BP_ATurnManager.BP_ATurnManager_C|GetTargets (Variables|Default|GetTurnManager)) (Variables|Default|GetThisPlayerNum))) (Variables|Default|GetTargetOffset)) false false))

(fn ReadEulerRotation
  (bind _playerrotation (Variables|Components|GetPlayerRotation))
  (bind _returnvalue (Class|PlayerRotationComponent|GetDeltaRotationEuler _playerrotation))
  (Rendering|Debug|DrawDebugLine :LineStart (Transformation|GetActorLocation) :LineEnd (Class|PlayerRotationComponent|GetDirectionfromCamera (Variables|Components|GetPlayerRotation)) :Duration 1e+01 :Thickness 1.0)
  (return (> (.X (Math|Vector|BreakVector _returnvalue)) 0.0) _returnvalue))

(fn PrintInputValueAssistFunct
  (bind _playerrotation (Variables|Components|GetPlayerRotation))
  (bind _returnvalue (Class|PlayerRotationComponent|GetRotationInputValue _playerrotation))
  (bind (_x _y _z) (Class|KismetMathLibrary|BreakQuat _returnvalue))
  (Development|PrintString (Utilities|String|ToString(Vector) (Math|Vector|MakeVector _x _y _z))))

(fn ChangeArrowForce
  (switch int (Variables|Default|GetSelectionSet) ; Set the force amount to launch the arrow based on the strength of the flex
    (:0
      (Variables|Default|SetForceValToPass 1.0))
    (:1
      (Variables|Default|SetForceValToPass 1.5))
    (:2
      (Variables|Default|SetForceValToPass 2.0))))

(fn OverlookShoulder
  (bind _returnvalue (Transformation|GetActorLocation))
  (bind (_x _y _z) (Math|Vector|BreakVector _returnvalue))
  (return (Math|Vector|MakeVector (+ _x (LocalVariables|GetXOffset)) (+ _y (LocalVariables|GetYOffset)) (+ _z (LocalVariables|GetZOffset)))))

(fn LinetraceIndicator
  (LocalVariables|SetPlayerPos (Transformation|GetWorldLocation (Variables|Components|GetPlayerObj)))
  (if (Variables|/Script/MinigameCore.MinigameBase|GetbIsPractice (Variables|/Game/Blueprints/ArcheryMinigameBlueprints/BP_ATurnManager.BP_ATurnManager_C|GetGameMode (Variables|Default|GetTurnManager)))
    (bind _outactors (Actor|GetAllActorswithTag "PracticeTarget"))
    (bind _asbp_atarget_parent (Utilities|Casting|CastToBP_ATargetParent (Utilities|Array|Get(acopy) _outactors)))
    (LocalVariables|SetTargetToMeasure _asbp_atarget_parent)
    (else
      (LocalVariables|SetTargetToMeasure (Variables|Default|GetAssignedTarget))))
  ;[0 0 0 1 12] Determine angle to point line at
  (if (> (Transformation|GetDistanceTo (LocalVariables|GetTargetToMeasure)) 1.09e+03) ; Check if beyond a certain distance to make angle positve or negative'
    (LocalVariables|SetAngleToTarget (* (Math|Float|Absolute(Float) (Math|Float|%(Float) (- (Transformation|GetDistanceTo (LocalVariables|GetTargetToMeasure)) 1.09e+03) 5e+01)) -1.0)) ; Further, should be negative
    (else
      (LocalVariables|SetAngleToTarget (Math|Float|Absolute(Float) (Math|Float|%(Float) (- (Transformation|GetDistanceTo (LocalVariables|GetTargetToMeasure)) 1.09e+03) 5e+01))) ; Closer, should be positive
    ))
  (bind _output_get (LocalVariables|SetEndPos (+ (* (+ (- (Transformation|GetWorldLocation (Variables|Default|GetForwardPos)) (Transformation|GetWorldLocation (Variables|Components|GetPlayerObj))) (Math|Vector|MakeVector (LocalVariables|GetAngleToTarget) (+ (.Y (Math|Vector|BreakVector (Transformation|GetActorForwardVector))) (Variables|Default|GetWind)) 0.0)) 1.5) (LocalVariables|GetPlayerPos))))
  ;[0 0 0 1 12] Linetrace method
  (CallFunction|ShootLineTraceBehavior (Utilities|Array|MakeArray (Variables|Default|GetArrowLandIndicatorLight) (Variables|Default|GetArrowLandIndicatorMedium) (Variables|Default|GetArrowLandIndicatorHeavy)) 0.0 _output_get (LocalVariables|GetPlayerPos) (LocalVariables|GetAngleToTarget))
  (CallFunction|ShootLineTraceBehavior (Utilities|Array|MakeArray (Variables|Default|GetArrowLandIndicatorMedium) (Variables|Default|GetArrowLandIndicatorHeavy)) 2e+01 (LocalVariables|GetEndPos) (LocalVariables|GetPlayerPos) (LocalVariables|GetAngleToTarget))
  (CallFunction|ShootLineTraceBehavior (Utilities|Array|MakeArray (Variables|Default|GetArrowLandIndicatorHeavy)) 5e+01 (LocalVariables|GetEndPos) (LocalVariables|GetPlayerPos) (LocalVariables|GetAngleToTarget)))

(fn RotatewithKeyboard
  (params (InputVal :type Vector%202D%20Structure))
  (bind _x (Math|Vector2D|BreakVector2D InputVal))
  (bind _returnvalue (Math|Rotator|MakeRotator 0.0 0.0 _x))
  (if (Variables|/Game/Blueprints/ArcheryMinigameBlueprints/BP_ATurnManager.BP_ATurnManager_C|GetinCutscene (Variables|Default|GetTurnManager)) ; Prevent input between player turn changes
    (Development|PrintString "Trying to rotate while in cutscene")
    (elif (Math|Float|InRange(Float) (+ (.Yaw (Math|Rotator|BreakRotator (Transformation|GetWorldRotation (Variables|Components|GetPlayerObj)))) _x) -45.0 45.0) ; This is supposed to limit rotation bw -45 to 45, not working right now
      (Transformation|AddRelativeRotation (Variables|Components|GetPlayerObj) _returnvalue false false)
      (Transformation|AddRelativeRotation (Variables|/Script/MinigameCore.MinigameCapture|GetSceneCapture (Variables|Default|GetCamera)) _returnvalue false false) ; Rotate camera with player
    )))

(fn SetIndicatorPosition
  (params (HitLocation :type Vector) (Angle :type Float%20%28double-precision%29) (WhichIndicator :type Array%20of%20Niagara%20Component%20Object%20References))
  (bind _returnvalue (Math|Vector|MakeVector -15.0 0.0 Angle))
  (bind _returnvalue_2 (+ HitLocation _returnvalue))
  (for _array_element WhichIndicator ; Run specifically if the line trace hits the target
    (Transformation|SetWorldLocation _array_element _returnvalue_2 false false) ; Set vfx position to point of collision
    (return _returnvalue_2))
  (Transformation|SetWorldLocation _array_element _returnvalue_2 false false) ; Set vfx position to point of collision
  (return _returnvalue_2))

(fn ShootLineTraceBehavior
  (params (ArrowIndicators :type Array%20of%20Niagara%20Component%20Object%20References) (LineDistanceAugment :type Float%20%28double-precision%29) (EndPos :type Vector) (PlayerPos :type Vector) (AngleToTarget :type Float%20%28double-precision%29))
  (bind (_x _y _z) (Math|Vector|BreakVector EndPos))
  (bind (_x_2 _y_2 _z_2) (Math|Vector|BreakVector EndPos))
  (bind (_outhit _returnvalue) (Collision|LineTraceByChannel PlayerPos (Math|Vector|MakeVector (+ _x 2e+01) _y _z) "TraceTypeQuery1" false 0 "Persistent"))
  (if _returnvalue ; Check if medium hit was valid
    (CallFunction|SetIndicatorPosition (.Location (Collision|BreakHitResult _outhit)) AngleToTarget ArrowIndicators)
    (else
      (CallFunction|SetIndicatorPosition (Math|Vector|MakeVector (+ _x_2 LineDistanceAugment) _y_2 _z_2) AngleToTarget (Utilities|Array|MakeArray (Utilities|Array|Get(acopy) ArrowIndicators))))))

(fn CalculateDestroyDistance
  (if (<= (Math|Vector|VectorLength (- (Transformation|GetWorldLocation (Variables|/Game/Blueprints/ArcheryMinigameBlueprints/BP_AArrow.BP_AArrow_C|GetArrowHead (Variables|Default|GetThisArrow))) (Transformation|GetWorldLocation (Variables|Default|GetForwardPos)))) (* (Math|Vector|VectorLength (- (Transformation|GetWorldLocation (Variables|Default|GetForwardPos)) (Transformation|GetWorldLocation (Variables|Components|GetPlayerObj)))) 0.75))
    (return true)
    (else
      (return false))))

(fn CheckifFirstPlayer
  (bind _outactors (Actor|GetAllActorsOfClass "BP_ArcheryPlayer_C"))
  (if (== (Utilities|Array|Length _outactors) 1)
    (return true)
    (else
      (return false))))

(fn SetPositioninPracticeMode
  (Transformation|SetActorLocation (Transformation|GetActorLocation (Variables|Default|GetPracticeTarget)) false false))