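; Arrow projectile for the archery minigame that flies toward the player's forward point, scoring on targets.
; A looping Timeline lerps the collider and head forward, while Tick adjusts velocity; the rise-and-fall arc logic is disconnected.
; Short forward and backward line traces each tick catch targets that fast arrows miss.
; Floor or range misses destroy it, passing the turn after the last arrow; `ArrowCleanupOnHit` leaves a placeholder arrow on the ring.
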(event OnComponentHit(Collider)
  (params (HitComponent :type Primitive%20Component%20Object%20Reference) (OtherActor :type Actor%20Object%20Reference) (OtherComp :type Primitive%20Component%20Object%20Reference) (NormalImpulse :type Vector :default "0, 0, 0") (Hit :type Hit%20Result%20Structure%20%28by%20ref%29))
  ;[0.1515 0.1823 0.02857] Collider hit - check for arrow/arrow collisions
  (if (Components|ComponentHasTag HitComponent "ArrowTag")
    (Collision|SetActorEnableCollision false) ; Prevent inital collision, realistically arrows would be thinner than the spheres, so collisions would happen less often and be more realistic
    (Utilities|FlowControl|Delay 0.2)
    (Collision|SetActorEnableCollision true)))

(event Custom|KeepMoving
  ;[0.1198 0 0.09719] On start
  (bind _newtrack_0 (Timeline|Timeline PlayFromStart) ; Start moving once arrow is instantaited
    (:Update
      (CallFunction|LaunchArrowForward (/ _newtrack_0 0.75)))
    (:Finished
      (CallFunction|KeepMoving))))

(event EventBeginPlay
  ;[0.1198 0 0.09719] On start
  (Utilities|FlowControl|Delay 0.01) ; Allow player to set
  (CallFunction|InitValues)
  (Variables|Default|SetForwardPos (Transformation|GetWorldLocation (Variables|/Game/Blueprints/ArcheryMinigameBlueprints/BP_ArcheryPlayer.BP_ArcheryPlayer_C|GetForwardPos (Variables|Default|GetPlayer))))
  (Components|Timeline|SetPlayRate (Variables|Default|GetTimeline) (Variables|Default|GetMultiplier))
  (bind _newtrack_0 (Timeline|Timeline Play) ; Start moving once arrow is instantaited
    (:Update
      (CallFunction|LaunchArrowForward (/ _newtrack_0 0.75)))
    (:Finished
      (CallFunction|KeepMoving))))

(event EventTick
  (params (DeltaSeconds :type Float%20%28single-precision%29))
  (bind _returnvalue (Transformation|GetVelocity))
  (bind _player (Variables|Default|GetPlayer))
  (bind _collider (Variables|Default|GetCollider))
  (bind _returnvalue_2 (Transformation|GetWorldLocation _collider))
  (bind (_x _y _z) (Math|Vector|BreakVector _returnvalue))
  (bind _forwardpos (Variables|/Game/Blueprints/ArcheryMinigameBlueprints/BP_ArcheryPlayer.BP_ArcheryPlayer_C|GetForwardPos _player))
  (bind _returnvalue_3 (Transformation|GetWorldLocation _forwardpos))
  (bind _returnvalue_4 (Math|Vector|Distance(Vector) _returnvalue_3 _returnvalue_2))
  ;[0.05288 0.2083 0.224] Event tick
  (bind (_hitprocessed _targetparent _targetset) (CallFunction|DetectTarget))
  (if (Variables|Default|GetHitTarget)
    (Default|EventParentRings _targetparent _targetset) ; Access none error??????
    (Transformation|SetActorLocation (Variables|Default|GetOffsetFromTargetRing) false false) ; Attach the arrow to the target if it hit the target
  )
  (if (Variables|Default|GetInMotion)
    (bind _velocityadditive (CallFunction|ApplyUpward/DownwardForce (Actor|GetGameTimeSinceCreation) (Variables|Default|GetMultiplier))) ; Currently using test strengths of flex
    (CallFunction|SetArrowVelocity _velocityadditive _y (> _z 0.0)) ; Vertical velocity should be connected to velocity additive, testing flat values
    (if (Variables|Default|GetHitTarget) ; if a target not detected
      (Development|PrintString "hit target true")
      (else
        (Utilities|IsValid _forwardpos ; if forward pos exists?
          (:Is%20Valid
            (if (not (< _returnvalue_4 9e+23)) ; Check distance from forward pos
              (Development|PrintString (Utilities|String|Append "Out of range by " (Utilities|String|ToString(Float) _returnvalue_4)))
              (CallFunction|DestroyArrow false))))))))

(event Collision|EventHit
  (params (MyComp :type Primitive%20Component%20Object%20Reference) (Other :type Actor%20Object%20Reference) (OtherComp :type Primitive%20Component%20Object%20Reference) (bSelfMoved :type Boolean) (HitLocation :type Vector :default "0, 0, 0") (HitNormal :type Vector :default "0, 0, 0") (NormalImpulse :type Vector :default "0, 0, 0") (Hit :type Hit%20Result%20Structure%20%28by%20ref%29))
  ;[0.05996 0.08355 0.2969] Event hit - check for arrow/floor collisons
  (if (Utilities|Enum|Equal(Enum) (Utilities|GetDisplayName Other) "Floor")
    (CallFunction|DestroyArrow true)))

(fn ConstructionScript)

(fn InitValues
  (bind _returnvalue (Actor|GetActorOfClass "/MinigameCore/Game/BP_MinigameCapture.BP_MinigameCapture_C")) ; Camera
  (Variables|Default|SetCamera _returnvalue)
  (bind _returnvalue_2 (Actor|GetActorOfClass "/Game/Blueprints/ArcheryMinigameBlueprints/BP_ATargetParent.BP_ATargetParent_C")) ; Target parent
  (Variables|Default|SetTargetTestForward _returnvalue_2)
  (bind _returnvalue_3 (Actor|GetActorOfClass "/Game/Blueprints/ArcheryMinigameBlueprints/BP_ATurnManager.BP_ATurnManager_C")) ; Turn manager
  (Variables|Default|SetTurnManager _returnvalue_3)
  (Transformation|SetActorRotation (Transformation|GetActorRotation (Variables|Default|GetPlayer)))
  (Variables|Default|SetInMotion true))

(fn LaunchArrowForward
  (params (Alpha :type Float%20%28single-precision%29))
  (bind _returnvalue (Transformation|GetActorLocation))
  (bind _forwardpos (Variables|Default|GetForwardPos))
  (bind _returnvalue_2 (Math|Vector|Lerp(Vector) _returnvalue _forwardpos 0.05))
  (Transformation|SetRelativeLocation (Variables|Default|GetCollider) _returnvalue_2 true false)
  (Transformation|SetRelativeLocation (Variables|Default|GetArrowHead) _returnvalue_2 false false)
  (return (+ (.Location (Math|Transform|BreakTransform (Transformation|GetRelativeTransform (Variables|/Script/MinigameCore.MinigameCapture|GetSceneCapture (Variables|Default|GetCamera))))) "1.000000,0.000000,0.000000")))

(fn ApplyWind
  (Physics|AddForce :Force (Math|Vector|MakeVector (Variables|/Game/Blueprints/ArcheryMinigameBlueprints/BP_ArcheryPlayer.BP_ArcheryPlayer_C|GetWind (Variables|Default|GetPlayer)) 0.0 0.0)))

(fn DestroyArrow
  (params (HitFloor :type Boolean))
  (if (Variables|Default|GetLastArrow) ; Whether this is the last arrow this player has or not
    (Development|PrintString "About to change player vira arrow")
    (Default|ChangePlayerTurn (Variables|Default|GetTurnManager))
    (CallFunction|ArrowCleanup)
    (else
      (CallFunction|ArrowCleanup))))

(fn SetLastArrow
  (Variables|Default|SetLastArrow true))

(fn ArrowCleanup
  (Development|PrintString "ARROW CLEANUP NOT HIT")
  (Variables|/Game/Blueprints/ArcheryMinigameBlueprints/BP_ArcheryPlayer.BP_ArcheryPlayer_C|SetThisArrow (Variables|Default|GetPlayer) 0)
  (Components|Activation|Activate (Variables|/Game/Blueprints/ArcheryMinigameBlueprints/BP_ArcheryPlayer.BP_ArcheryPlayer_C|GetArrowDestroyed (Variables|Default|GetPlayer)) false)
  (Actor|DestroyActor))

(fn ApplyUpward/DownwardForce
  (params (SecondsPassed :type Float%20%28double-precision%29) (StrengthOfFlex :type Float%20%28double-precision%29))
  (return (LocalVariables|GetAddToVelocity)))

(fn SetArrowVelocity
  (params (VerticalVelocity :type Vector) (ZVelocity :type Float%20%28double-precision%29) (IsZValid :type Boolean))
  (if IsZValid
    (Physics|SetPhysicsLinearVelocity (Variables|Default|GetCollider) (+ VerticalVelocity (Transformation|GetVelocity)) false "None") ; Add the upward/downward movement to velocity if already moving
    (else
      (Utilities|IsValid self
        (:Is%20Valid
          (Physics|SetPhysicsLinearVelocity (Variables|Default|GetArrowHead) (+ VerticalVelocity (Transformation|GetVelocity) "100.000000,0.000000,0.000000") true "None") ; Force object to move when stopped,  may need a more practical solution
        ))))
  (return (> ZVelocity 0.0)))

(fn ArrowCleanuponHit
  (params (TargetHit :type BP%20A%20Target%20Object%20Reference) (HitLocation :type Vector))
  (bind _returnvalue (Game|SpawnActorfromClass "/Game/Blueprints/ArcheryMinigameBlueprints/BP_AArrowPlaceholder.BP_AArrowPlaceholder_C" (Math|Transform|MakeTransform HitLocation) "AlwaysSpawn" "MultiplyWithRoot" 0 0)) ; Spawn the defunct arrow
  (Transformation|AttachComponentToComponent _returnvalue (Variables|/Game/Blueprints/ArcheryMinigameBlueprints/BP_ATarget.BP_ATarget_C|GetTargetRing TargetHit) "None" "SnapToTarget" "KeepRelative" "KeepRelative" true) ; Attach to target ring where hit
  (Physics|SetSimulatePhysics (Variables|/Game/Blueprints/ArcheryMinigameBlueprints/BP_AArrowPlaceholder.BP_AArrowPlaceholder_C|GetArrowHead _returnvalue) false) ; Ensure physics are not enabled
  (Components|Activation|Activate (Variables|/Game/Blueprints/ArcheryMinigameBlueprints/BP_AArrowPlaceholder.BP_AArrowPlaceholder_C|GetHitVFX _returnvalue) false)
  (CallFunction|ArrowCleanup) ; Destroy active arrow
)

(fn ManageColorRotation
  (params (TargetArray :type Array%20of%20Linear%20Color%20Structures))
  (Math|Integer|IncrementInt (Variables|Default|GetTempColorRotator)
    (:%20%20
      (if (>= (Variables|Default|GetTempColorRotator) (Utilities|Array|Length TargetArray))
        (Variables|Default|SetTempColorRotator 0)))))

(fn DetectTarget
  (bind _returnvalue (Transformation|GetActorLocation))
  (bind _returnvalue_2 (Transformation|GetActorLocation))
  (bind _array (Utilities|Array|MakeArray "ObjectTypeQuery2"))
  (if (not (Variables|Default|GetHitTarget))
    (bind (_outhit _returnvalue_3) (Collision|LineTraceForObjects _returnvalue (+ _returnvalue "5.000000,0.000000,0.000000") _array false 0 "Persistent" true "(R=1.000000,G=0.000000,B=0.000000,A=1.000000)" "(R=0.000000,G=1.000000,B=0.000000,A=1.000000)" 1e+18)) ; Forward ray
    (if _returnvalue_3
      (LocalVariables|SetHitObj _outhit)
      (if (Class|GameplayStatics|ObjectIsA (.HitActor (Collision|BreakHitResult (LocalVariables|GetHitObj))) "/Game/Blueprints/ArcheryMinigameBlueprints/BP_ATarget.BP_ATarget_C") :!label _label
        (bind _asbp_atarget (Utilities|Casting|CastToBP_ATarget (.HitActor (Collision|BreakHitResult (LocalVariables|GetHitObj))))) ; Converts to first target?
        (LocalVariables|SetHitLocal (.Location (Collision|BreakHitResult (LocalVariables|GetHitObj))))
        (LocalVariables|SetTargetDetected _asbp_atarget)
        (Variables|Default|SetHitTarget true)
        (Default|AddPointsonTargetHit (LocalVariables|GetTargetDetected) self (LocalVariables|GetHitLocal))
        (return true (Variables|/Game/Blueprints/ArcheryMinigameBlueprints/BP_ATarget.BP_ATarget_C|GetTargetParent (LocalVariables|GetTargetDetected)) (LocalVariables|GetTargetDetected))
        (else
          (return false 0 0)))
      (else
        (bind (_outhit_2 _returnvalue_4) (Collision|LineTraceForObjects _returnvalue_2 (- _returnvalue_2 "5.000000,0.000000,0.000000") _array false 0 "Persistent" true "(R=1.000000,G=0.000000,B=0.000000,A=1.000000)" "(R=0.000000,G=1.000000,B=0.000000,A=1.000000)" 1e+15)) ; Backward ray
        (if _returnvalue_4
          (LocalVariables|SetHitObj _outhit_2)
          (goto _label))))))