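; End cutscene manager for the archery minigame that announces the winning player before ending the cutscene.
; On start, it shows the GameMode winner's number on the turn UI, holds briefly, fades it out, then calls EndCutscene.
; InitValues finds the BP_APlayerTurnUI widget by class search and prints debug messages.
; SetCutsceneText drives its text and fade animations, while CheckUIOpacity and SetUIText are empty stubs.
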(event EventOnStartCutscene
  (params (Minigame :type Minigame%20Base%20Object%20Reference))
  (CallFunction|SetCutsceneText (Utilities|String|MakeLiteralString (Utilities|String|Append "Player " (Utilities|String|ToString(Integer) (+ (Variables|/Script/MinigameCore.MinigamePlayer|GetPlayerNumber (Variables|/Game/Blueprints/ArcheryMinigameBlueprints/BP_ArcheryGamemode.BP_ArcheryGamemode_C|GetWinner (Variables|Default|GetGameMode))) 1)) " Wins!")) false)
  (Utilities|FlowControl|Delay Minigame 3.0)
  (CallFunction|SetCutsceneText "" true)
  (Utilities|FlowControl|Delay Minigame 1.0)
  (Class|MinigameCutsceneManager|EndCutscene))

(fn CheckUIOpacity
  (params (FadeIn :type Boolean)))

(fn SetUIText
  (params (TextString :type String) (OpacityChange :type Float%20%28double-precision%29)))

(fn SetCutsceneText
  (params (UIText :type String) (ShouldFadeOut :type Boolean))
  (bind _turnui (Variables|Default|GetTurnUI))
  (bind _turnui_2 (Variables|Default|GetTurnUI))
  (if ShouldFadeOut
    (UserInterface|Animation|PlayAnimation _turnui (Variables|/Game/Blueprints/ArcheryMinigameBlueprints/BP_APlayerTurnUI.BP_APlayerTurnUI_C|GetFadeOut _turnui) 0.0 1 "Forward" 1.0 false)
    (else
      (Variables|/Script/UMG.TextBlock|SetText (Variables|/Game/Blueprints/ArcheryMinigameBlueprints/BP_APlayerTurnUI.BP_APlayerTurnUI_C|GetPlayerTurnID (Variables|Default|GetTurnUI)) (Utilities|Text|ToText(String) UIText))
      (UserInterface|Animation|PlayAnimation _turnui_2 (Variables|/Game/Blueprints/ArcheryMinigameBlueprints/BP_APlayerTurnUI.BP_APlayerTurnUI_C|GetFadeIn _turnui_2) 0.0 1 "Forward" 1.0 false))))

(fn InitValues
  (Development|PrintString 0 "END CUTSCENE BEGAN" true true "(R=0.000000,G=1.000000,B=0.027641,A=1.000000)" 5.0)
  (bind _foundwidgets (Widget|GetAllWidgetsOfClass (Class|MinigameCutsceneManager|GetWorld) "/Game/Blueprints/ArcheryMinigameBlueprints/BP_APlayerTurnUI.BP_APlayerTurnUI_C")) ; Stops here
  (Utilities|IsValid (Utilities|Array|Get(acopy) _foundwidgets)
    (:Is%20Valid
      (Development|PrintString 0 (Utilities|GetDisplayName (Utilities|Array|Get(acopy) _foundwidgets)))
      (Variables|Default|SetTurnUI (Utilities|Array|Get(acopy) _foundwidgets)))
    (:Is%20Not%20Valid
      (Development|PrintString 0 "cannot access UI"))))