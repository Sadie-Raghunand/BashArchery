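; Turn manager for the archery minigame that moves the camera from player to player and announces whose turn it is.
; ChangePlayerTurn advances the index, automatically on a Tick timer in practice mode, and ends real games after the last player.
; A MoveCamera timeline lerps the manager and capture camera to an over-the-shoulder offset, triggering turn text fades.
; InitValues caches references and sets target visibility.
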(event Custom|StopCamMovement
  ;[0.15 0.03051 0.03216 0.5] Tick
  (bind _newtrack_0 (Timeline|MoveCamera Stop) ; Move camera to the side to position in front of next player's target
    (:Update
      (if (< (Variables|Default|GetPlayerTurn) (Utilities|Array|Length (Variables|Default|GetPlayers))) ; Check to see if there are any more players' whose turn it will be
        (bind _cameraendpos (CallFunction|OverlookShoulder))
        (CallFunction|MoveCameratoNextPos _newtrack_0 _cameraendpos)
        (if (not (== (Variables|Default|GetPlayerTurn) 0)) ; Player 0's UI already handled by cutscene
          (CallFunction|ChangeCutsceneStatus) ; Is here the issue for the cutscene bool never changing?
          (Default|CallFadeUI (Variables|Default|GetGameMode) false (Utilities|String|MakeLiteralString (Utilities|String|Append "Player " (Utilities|String|ToString(Integer) (+ (Variables|Default|GetPlayerTurn) 1)) "'s Turn!")))
          (Utilities|FlowControl|Delay 3.0)
          (Default|CallFadeUI (Variables|Default|GetGameMode) true)
          (CallFunction|ChangePlayerTurnUI "" true)
          (CallFunction|ChangeCutsceneStatus))
        (elif (not (Variables|/Script/MinigameCore.MinigameBase|GetbIsPractice (Variables|Default|GetGameMode)))
          (Class|MinigameBase|EndGame (Variables|Default|GetGameMode)))))))

(event EventBeginPlay
  ;[0.07824 0.09238 0.15 0.5] Begin play
  (bind _returnvalue (Actor|GetActorOfClass "/Game/Blueprints/ArcheryMinigameBlueprints/BP_ArcheryGamemode.BP_ArcheryGamemode_C"))
  (bind _output_get (Variables|Default|SetGameMode _returnvalue))
  (if (Variables|/Script/MinigameCore.MinigameBase|GetbIsPractice _output_get)
    (Utilities|FlowControl|Delay 0.5) ; Prevent move cam from happening before players are spawned in
    (CallFunction|InitValues)
    ;[0.15 0.03051 0.03216 0.5] Tick
    (bind _newtrack_0 (Timeline|MoveCamera Play) ; Move camera to the side to position in front of next player's target
      (:Update
        (if (< (Variables|Default|GetPlayerTurn) (Utilities|Array|Length (Variables|Default|GetPlayers))) ; Check to see if there are any more players' whose turn it will be
          (bind _cameraendpos (CallFunction|OverlookShoulder))
          (CallFunction|MoveCameratoNextPos _newtrack_0 _cameraendpos)
          (if (not (== (Variables|Default|GetPlayerTurn) 0)) ; Player 0's UI already handled by cutscene
            (CallFunction|ChangeCutsceneStatus) ; Is here the issue for the cutscene bool never changing?
            (Default|CallFadeUI (Variables|Default|GetGameMode) false (Utilities|String|MakeLiteralString (Utilities|String|Append "Player " (Utilities|String|ToString(Integer) (+ (Variables|Default|GetPlayerTurn) 1)) "'s Turn!")))
            (Utilities|FlowControl|Delay 3.0)
            (Default|CallFadeUI (Variables|Default|GetGameMode) true)
            (CallFunction|ChangePlayerTurnUI "" true)
            (CallFunction|ChangeCutsceneStatus))
          (elif (not (Variables|/Script/MinigameCore.MinigameBase|GetbIsPractice (Variables|Default|GetGameMode)))
            (Class|MinigameBase|EndGame (Variables|Default|GetGameMode))))))))

(event EventTick
  (params (DeltaSeconds :type Float%20%28single-precision%29))
  ;[0.15 0.03051 0.03216 0.5] Tick
  (Variables|Default|SetTimeSinceTurn (+ DeltaSeconds (Variables|Default|GetTimeSinceTurn)))
  (CallFunction|SwitchonTimerPractice)
  (if (Variables|Default|GetMoving)
    (bind _newtrack_0 (Timeline|MoveCamera Play) ; Move camera to the side to position in front of next player's target
      (:Update
        (if (< (Variables|Default|GetPlayerTurn) (Utilities|Array|Length (Variables|Default|GetPlayers))) ; Check to see if there are any more players' whose turn it will be
          (bind _cameraendpos (CallFunction|OverlookShoulder))
          (CallFunction|MoveCameratoNextPos _newtrack_0 _cameraendpos)
          (if (not (== (Variables|Default|GetPlayerTurn) 0)) ; Player 0's UI already handled by cutscene
            (CallFunction|ChangeCutsceneStatus) ; Is here the issue for the cutscene bool never changing?
            (Default|CallFadeUI (Variables|Default|GetGameMode) false (Utilities|String|MakeLiteralString (Utilities|String|Append "Player " (Utilities|String|ToString(Integer) (+ (Variables|Default|GetPlayerTurn) 1)) "'s Turn!")))
            (Utilities|FlowControl|Delay 3.0)
            (Default|CallFadeUI (Variables|Default|GetGameMode) true)
            (CallFunction|ChangePlayerTurnUI "" true)
            (CallFunction|ChangeCutsceneStatus))
          (elif (not (Variables|/Script/MinigameCore.MinigameBase|GetbIsPractice (Variables|Default|GetGameMode)))
            (Class|MinigameBase|EndGame (Variables|Default|GetGameMode))))))))

(fn ConstructionScript)

(fn ChangePlayerTurn
  (Development|PrintString "Change player turn called")
  (if (>= (Variables|Default|GetPlayerTurn) (Utilities|Array|Length (Variables|Default|GetPlayers))) ; f true, end minigame, if false, move to next player
    (Development|PrintString "No more players ")
    (if (Variables|/Script/MinigameCore.MinigameBase|GetbIsPractice (Variables|Default|GetGameMode))
      (Development|PrintString "Go back to player 1") ; Game should reset
      (else
        (Class|MinigameBase|EndGame (Variables|Default|GetGameMode))))
    (else
      (bind _result (Math|Integer|IncrementInt (Variables|Default|GetPlayerTurn))
        (:%20%20
          (Variables|Default|SetPlayerTurn _result)
          (Development|PrintString "Setting moving to true")
          (Variables|Default|SetMoving true)
          (Variables|Default|SetInPos false))))))

(fn InitValues
  (bind _returnvalue (Actor|GetActorOfClass "/MinigameCore/Game/BP_MinigameCapture.BP_MinigameCapture_C"))
  (Variables|Default|SetCamera _returnvalue)
  (bind _returnvalue_2 (Actor|GetActorOfClass "/Game/Blueprints/ArcheryMinigameBlueprints/BP_ArcheryGamemode.BP_ArcheryGamemode_C"))
  (bind _output_get (Variables|Default|SetGameMode _returnvalue_2))
  (if (Variables|/Script/MinigameCore.MinigameBase|GetbIsPractice _output_get)
    _
    (else
      (Variables|Default|SetMoving true)))
  (bind _arrayindex (Utilities|Array|ReverseforEachLoop (Variables|Default|GetTargets)) ; Set targets not assigned to a player inactive
    (:LoopBody
      (if (not (> (Variables|Default|GetTurnsTotal) _arrayindex))
        (Rendering|SetActorHiddenInGame (Utilities|Array|Get(acopy) (Variables|Default|GetTargets) _arrayindex) true)
        (for _array_element (Variables|/Game/Blueprints/ArcheryMinigameBlueprints/BP_ATargetParent.BP_ATargetParent_C|GetTargetRings (Utilities|Array|Get(acopy) (Variables|Default|GetTargets) _arrayindex)) ; Set rings inactive as well
          (Rendering|SetActorHiddenInGame _array_element true)
          (Transformation|SetActorRotation (Variables|Default|GetCamera))
          (bind _foundwidgets (Widget|GetAllWidgetsOfClass "/Game/Blueprints/ArcheryMinigameBlueprints/UI/Old/BP_APlayerTurnUI.BP_APlayerTurnUI_C" true))
          (Variables|Default|SetPlayerTurnUI (Utilities|Array|Get(acopy) _foundwidgets))
          (CallFunction|SetInactiveandActiveTargets))
        (bind _foundwidgets_2 (Widget|GetAllWidgetsOfClass "/Game/Blueprints/ArcheryMinigameBlueprints/UI/Old/BP_APlayerTurnUI.BP_APlayerTurnUI_C" true))
        (Variables|Default|SetPlayerTurnUI (Utilities|Array|Get(acopy) _foundwidgets_2))
        (CallFunction|SetInactiveandActiveTargets)))))

(fn MoveCameratoNextPos
  (params (Alpha :type Float%20%28single-precision%29) (CameraPos :type Vector))
  (bind _players (Variables|Default|GetPlayers))
  (bind _playerturn (Variables|Default|GetPlayerTurn))
  (bind _output (Utilities|Array|Get(acopy) _players _playerturn))
  (Utilities|IsValid _output
    (:Is%20Valid
      (Transformation|SetWorldLocation (Variables|Default|GetDefaultSceneRoot) (Math|Vector|Lerp(Vector) (Transformation|GetActorLocation) (Transformation|GetActorLocation _output) Alpha) false false) ; Set this position
      (Transformation|SetWorldLocation (Variables|/Script/Engine.Actor|GetRootComponent (Variables|Default|GetCamera)) CameraPos false false) ; Set camera position
      (Transformation|SetActorRotation (Variables|Default|GetCamera)) ; Force no rotation on camera
    )))

(fn ResetThisGame
  (Default|OnGameResetEvent (Variables|Default|GetGameMode)) ; Set camera position back to begining position
  (Variables|Default|SetMoving true))

(fn CheckinPosition
  (if (== (Transformation|GetActorTransform) (Transformation|GetActorTransform (Utilities|Array|Get(acopy) (Variables|Default|GetPlayers) (Variables|Default|GetPlayerTurn))))
    (Variables|Default|SetInPos true)))

(fn RotateTowardsTarget
  (Transformation|SetActorRotation (Variables|Default|GetCamera) (Math|Rotator|FindLookatRotation (Math|Rotator|GetRotationXVector (Transformation|GetActorRotation)) (Transformation|GetActorLocation (Utilities|Array|Get(acopy) (Variables|Default|GetTargets) (Variables|Default|GetPlayerTurn)))))
  (Variables|Default|SetMoving false)
  (Development|PrintString "Cam NOT in pos" true true "(R=0.000000,G=0.660000,B=1.000000,A=1.000000)" 0.5))

(fn OnEndMovement
  (Development|PrintString "IN POSITION"))

(fn OverlookShoulder
  (bind _players (Variables|Default|GetPlayers))
  (bind _playerturn (Variables|Default|GetPlayerTurn))
  (bind _output (Utilities|Array|Get(acopy) _players _playerturn))
  (bind _returnvalue (Transformation|GetActorLocation _output))
  (bind (_x _y _z) (Math|Vector|BreakVector _returnvalue))
  (Utilities|IsValid _output
    (:Is%20Valid
      (return (Math|Vector|MakeVector (+ _x (LocalVariables|GetXOffset)) (+ _y (LocalVariables|GetYOffset)) (+ _z (LocalVariables|GetZOffset)))))
    (:Is%20Not%20Valid
      (return "0, 0, 0"))))

(fn ChangePlayerTurnUI
  (params (UIText :type String) (ShouldFadeOut :type Boolean))
  (bind _playerturnui (Variables|Default|GetPlayerTurnUI))
  (bind _playerturnui_2 (Variables|Default|GetPlayerTurnUI))
  (if ShouldFadeOut
    (UserInterface|Animation|PlayAnimation _playerturnui_2 (Variables|/Game/Blueprints/ArcheryMinigameBlueprints/UI/Old/BP_APlayerTurnUI.BP_APlayerTurnUI_C|GetFadeOut _playerturnui_2) 0.0 1 "Forward" 1.0 false)
    (else
      (Variables|/Script/UMG.TextBlock|SetText (Variables|/Game/Blueprints/ArcheryMinigameBlueprints/UI/Old/BP_APlayerTurnUI.BP_APlayerTurnUI_C|GetPlayerTurnID (Variables|Default|GetPlayerTurnUI)) (Utilities|Text|ToText(String) UIText))
      (UserInterface|Animation|PlayAnimation _playerturnui (Variables|/Game/Blueprints/ArcheryMinigameBlueprints/UI/Old/BP_APlayerTurnUI.BP_APlayerTurnUI_C|GetFadeIn _playerturnui) 0.0 1 "Forward" 1.0 false))))

(fn ChangeCutsceneStatus
  (if (Variables|/Script/MinigameCore.MinigameBase|GetbIsPractice (Variables|Default|GetGameMode))
    (Development|PrintString "In practice trying to change in cutscene")
    (else
      (bind _output_get (Variables|Default|SetinCutscene (not (Variables|Default|GetinCutscene))))
      (Development|PrintString (Utilities|String|Append "In cutscene changed to " (Utilities|String|ToString(Boolean) _output_get)) true true "(R=0.024465,G=0.526042,B=0.044584,A=1.000000)"))))

(fn SetInactiveandActiveTargets
  (for _array_element (Variables|Default|GetTargets) ; Is not practice mode, Set targets that are not the practice target invisible
    (for _array_element_2 (Variables|/Game/Blueprints/ArcheryMinigameBlueprints/BP_ATargetParent.BP_ATargetParent_C|GetTargetRings _array_element)
      (Rendering|SetActorHiddenInGame _array_element_2 false))
    (Rendering|SetActorHiddenInGame _array_element false)))

(fn SwitchonTimerPractice
  (if (Variables|/Script/MinigameCore.MinigameBase|GetbIsPractice (Variables|Default|GetGameMode))
    (if (>= (Variables|Default|GetTimeSinceTurn) (LocalVariables|GetMaxSeconds))
      (CallFunction|ChangePlayerTurn)
      (Variables|Default|SetTimeSinceTurn 0.0))))