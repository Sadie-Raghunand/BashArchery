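; Intro cutscene manager for the archery minigame that plays the opening "Start!" and "Player 1's Turn!" announcements.
; On start, it looks up the turn UI, turn manager and capture camera, then places the camera and triggers the turn manager's camera movement.
; Delayed widget fade animations sequence the text, then all arrows are destroyed before the cutscene ends.
; Manual camera-lerp and text-opacity helpers are defined but not called here.
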(event EventOnStartCutscene
  (params (Minigame :type Minigame%20Base%20Object%20Reference))
  (CallFunction|InitValues)
  (Transformation|SetActorLocation (Variables|Default|GetCamera) (Variables|/Game/Blueprints/ArcheryMinigameBlueprints/BP_ATurnManager.BP_ATurnManager_C|GetCameraCutsceneStartPos (Variables|Default|GetTurnManager)) false false)
  (Default|StartCutsceneCamMovement (Variables|Default|GetTurnManager))
  ;[0.15 0.15 0.15 0.5] Fade in/out w animation
  (CallFunction|SetCutsceneText "Start!" false)
  (Utilities|FlowControl|Delay Minigame 3.0)
  (CallFunction|SetCutsceneText "" true)
  (Utilities|FlowControl|Delay Minigame 1.0)
  (CallFunction|SetCutsceneText "Player 1's Turn!" false)
  (Utilities|FlowControl|Delay Minigame 3.0)
  (CallFunction|SetCutsceneText "" true)
  (Utilities|FlowControl|Delay Minigame 1.0)
  (bind _outactors (Actor|GetAllActorsOfClass Minigame "/Game/Blueprints/ArcheryMinigameBlueprints/BP_AArrow.BP_AArrow_C")) ; Appears to not be working
  (for _array_element _outactors
    (Actor|DestroyActor _array_element))
  (Class|MinigameCutsceneManager|EndCutscene))

(fn MoveCameraIntoAcheryRange
  (Transformation|SetActorLocation (Variables|Default|GetCamera) (Math|Vector|Lerp(Vector) (Transformation|GetWorldLocation (Variables|/Script/MinigameCore.MinigameCapture|GetSceneCapture (Variables|Default|GetCamera))) (Transformation|GetActorForwardVector (Variables|Default|GetCamera)) 0.01) false false))

(fn InitValues
  (bind _returnvalue (Class|MinigameCutsceneManager|GetWorld))
  (Development|PrintString 0 "START CUTSCENE BEGAN" true true "(R=0.000000,G=1.000000,B=0.027641,A=1.000000)" 5.0)
  (bind _foundwidgets (Widget|GetAllWidgetsOfClass _returnvalue "/Game/Blueprints/ArcheryMinigameBlueprints/BP_APlayerTurnUI.BP_APlayerTurnUI_C")) ; Stops here
  (Utilities|IsValid (Utilities|Array|Get(acopy) _foundwidgets)
    (:Is%20Valid
      (Development|PrintString 0 (Utilities|GetDisplayName (Utilities|Array|Get(acopy) _foundwidgets)))
      (Variables|Default|SetTurnUI (Utilities|Array|Get(acopy) _foundwidgets))
      (bind _returnvalue_2 (Actor|GetActorOfClass _returnvalue "/Game/Blueprints/ArcheryMinigameBlueprints/BP_ATurnManager.BP_ATurnManager_C"))
      (Variables|Default|SetTurnManager _returnvalue_2)
      (bind _returnvalue_3 (Actor|GetActorOfClass _returnvalue "/MinigameCore/Game/BP_MinigameCapture.BP_MinigameCapture_C"))
      (Variables|Default|SetCamera _returnvalue_3))
    (:Is%20Not%20Valid
      (Development|PrintString 0 "cannot access UI"))))

(fn SetUIText
  (params (TextString :type String) (OpacityChange :type Float%20%28double-precision%29))
  (bind _turnui (Variables|Default|GetTurnUI))
  (bind _playerturnid (Variables|/Game/Blueprints/ArcheryMinigameBlueprints/BP_APlayerTurnUI.BP_APlayerTurnUI_C|GetPlayerTurnID _turnui))
  (Variables|/Script/UMG.TextBlock|SetText _playerturnid (Utilities|Text|ToText(String) TextString))
  (Appearance|SetColorandOpacity (Variables|/Game/Blueprints/ArcheryMinigameBlueprints/BP_APlayerTurnUI.BP_APlayerTurnUI_C|GetPlayerTurnID (Variables|Default|GetTurnUI)) (Utilities|Struct|MakeSlateColor (Math|Color|MakeColor 0.0 0.0 0.0 (+ (.A (Math|Color|BreakColor (.SpecifiedColor (Utilities|Struct|BreakSlateColor (Variables|/Script/UMG.TextBlock|GetColorAndOpacity _playerturnid))))) OpacityChange))) :!class /Script/UMG.TextBlock))

(fn CheckUIOpacity
  (params (FadeIn :type Boolean))
  (bind _turnui (Variables|Default|GetTurnUI))
  (bind _playerturnid (Variables|/Game/Blueprints/ArcheryMinigameBlueprints/BP_APlayerTurnUI.BP_APlayerTurnUI_C|GetPlayerTurnID _turnui))
  (bind _colorandopacity (Variables|/Script/UMG.TextBlock|GetColorAndOpacity _playerturnid))
  (bind _specifiedcolor (Utilities|Struct|BreakSlateColor _colorandopacity))
  (bind _a (Utilities|Struct|BreakLinearColor _specifiedcolor))
  (Variables|Default|SetFadeFinished false)
  (if FadeIn
    (if (not (< _a 1.0)) ; Check if opaque
      (Variables|Default|SetFadeFinished true))
    (elif (not (> _a 0.0)) ; Check if transparent
      (Variables|Default|SetFadeFinished true))))

(fn SetCutsceneText
  (params (TextForUI :type String) (EraseText :type Boolean))
  (bind _turnui (Variables|Default|GetTurnUI))
  (bind _turnui_2 (Variables|Default|GetTurnUI))
  (if EraseText
    (UserInterface|Animation|PlayAnimation _turnui (Variables|/Game/Blueprints/ArcheryMinigameBlueprints/BP_APlayerTurnUI.BP_APlayerTurnUI_C|GetFadeOut _turnui) 0.0 1 "Forward" 1.0 false)
    (else
      (Variables|/Script/UMG.TextBlock|SetText (Variables|/Game/Blueprints/ArcheryMinigameBlueprints/BP_APlayerTurnUI.BP_APlayerTurnUI_C|GetPlayerTurnID (Variables|Default|GetTurnUI)) (Utilities|Text|ToText(String) TextForUI))
      (UserInterface|Animation|PlayAnimation _turnui_2 (Variables|/Game/Blueprints/ArcheryMinigameBlueprints/BP_APlayerTurnUI.BP_APlayerTurnUI_C|GetFadeIn _turnui_2) 0.0 1 "Forward" 1.0 false))))