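; Parent archery target actor that scores arrow hits and jumps to a new random spot.
; On arrow overlap, distance from center picks one of four point rings, scored through the gamemode's point counter and UI only for the assigned target or in practice.
; A dynamic-material highlight scales to the scored ring and fades in and out in timed steps.
; Each hit relocates the root within a box, briefly detaching the teleport VFX.
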(event OnComponentBeginOverlap(TestRingCollision)
  (params (OverlappedComponent :type Primitive%20Component%20Object%20Reference) (OtherActor :type Actor%20Object%20Reference) (OtherComp :type Primitive%20Component%20Object%20Reference) (OtherBodyIndex :type Integer) (bFromSweep :type Boolean) (SweepResult :type Hit%20Result%20Structure%20%28by%20ref%29))
  (Class|KismetSystemLibrary|IsObjectOfSoftClass OtherActor "/Game/Blueprints/ArcheryMinigameBlueprints/BP_AArrow.BP_AArrow_C"
    (:True
      (bind _asbp_aarrow (Utilities|Casting|CastToBP_AArrow OtherActor))
      (bind (_hitlocation _distance) (CallFunction|CalculateDistancefromCenter _asbp_aarrow))
      (if (> _distance 6e+01) ; Split between ring 1/2 and 3/4
        (if (> _distance 75.0) ; Split between ring 3 and 4
          (bind _pointsassigned (CallFunction|AssignPointsBasedonDistance 3 _asbp_aarrow _hitlocation 1))
          (CallFunction|EventHighlightHitRing true _pointsassigned) ; Make scale change a global variable?
          (else
            (bind _pointsassigned_2 (CallFunction|AssignPointsBasedonDistance 2 _asbp_aarrow _hitlocation 2))
            (CallFunction|EventHighlightHitRing true _pointsassigned_2) ; Make scale change a global variable?
          ))
        (elif (> _distance 45.0) ; Split between ring 1 and 2
          (bind _pointsassigned_3 (CallFunction|AssignPointsBasedonDistance 1 _asbp_aarrow _hitlocation 3))
          (CallFunction|EventHighlightHitRing true _pointsassigned_3) ; Make scale change a global variable?
          (else
            (bind _pointsassigned_4 (CallFunction|AssignPointsBasedonDistance 0 _asbp_aarrow _hitlocation 4))
            (CallFunction|EventHighlightHitRing true _pointsassigned_4) ; Make scale change a global variable?
          )))
      (CallFunction|ChangeLocation)
      (Utilities|FlowControl|Delay 1.75)
      (Transformation|AttachComponentToComponent (Variables|Default|GetTeleportVFX) (Variables|Default|GetDefaultSceneRoot) "None" "KeepRelative" "KeepRelative" "KeepRelative" true)
      (Transformation|SetRelativeLocation (Variables|Default|GetTeleportVFX) "0.000000,0.000000,-260.000000" false false))))

(event Custom|Event_HighlightHitRing
  (params (FadeIn :type Boolean) (Points :type Integer))
  ;[0.07253 0.09854 0.15 0.5] Highlight ring hit
  (CallFunction|CalculateHighlightScale Points)
  (CallFunction|HighlightRing FadeIn)
  (Utilities|FlowControl|Delay 0.1)
  (CallFunction|HighlightRing FadeIn)
  (Utilities|FlowControl|Delay 0.1)
  (CallFunction|HighlightRing FadeIn)
  (Utilities|FlowControl|Delay 0.1)
  (CallFunction|HighlightRing FadeIn)
  (Utilities|FlowControl|Delay 0.1)
  (CallFunction|HighlightRing FadeIn)
  (Utilities|FlowControl|Delay 0.1)
  (CallFunction|HighlightRing FadeIn)
  (Utilities|FlowControl|Delay 0.1)
  (CallFunction|HighlightRing FadeIn)
  (Utilities|FlowControl|Delay 0.1)
  (CallFunction|HighlightRing FadeIn)
  (Utilities|FlowControl|Delay 0.1)
  (CallFunction|HighlightRing FadeIn)
  (Utilities|FlowControl|Delay 0.1)
  (CallFunction|HighlightRing FadeIn)
  (if FadeIn
    (CallFunction|EventHighlightHitRing false Points)))

(event EventBeginPlay
  (bind _highlight (Variables|Default|GetHighlight))
  (Variables|Default|SetCenterPos (+ (Transformation|GetActorLocation) "1000.000000,0.000000,0.000000"))
  (bind _returnvalue (Actor|GetActorOfClass "/Game/Blueprints/ArcheryMinigameBlueprints/BP_ArcheryGamemode.BP_ArcheryGamemode_C"))
  (Variables|Default|SetGameModeReference _returnvalue)
  (Input|EnableInput 0)
  (bind _returnvalue_2 (Rendering|Material|CreateDynamicMaterialInstance _highlight 0 (Rendering|Material|GetMaterial _highlight 0) "None" :!class /Script/Engine.PrimitiveComponent))
  (Variables|Default|SetHighlightMat _returnvalue_2))

(fn ConstructionScript)

(fn ChangeLocation
  (Components|Activation|Activate (Variables|Default|GetTeleportVFX) false) ; Can't follow target though\n\nChange position of everything else, delay this?
  (Transformation|DetachFromComponent (Variables|Default|GetTeleportVFX) "KeepWorld" "KeepWorld" "KeepWorld" true)
  (Transformation|SetWorldLocation (Variables|Default|GetDefaultSceneRoot) (Math|Random|RandomPointinBoundingBox (Variables|Default|GetCenterPos) "75.000000,200.000000,0.000000") false false) ; Change parent location
)

(fn PlayFeedback
  (Components|Activation|Activate (Variables|Default|GetHitTargetFeedback) false))

(fn AssignPointsBasedonDistance
  (params (Index :type Integer) (ArrowHit :type BP%20A%20Arrow%20Object%20Reference) (ArrowLocationOnHit :type Vector) (Points :type Integer))
  (bind _gamemodereference (Variables|Default|GetGameModeReference))
  (bind _turnmanager (Variables|/Game/Blueprints/ArcheryMinigameBlueprints/BP_ArcheryGamemode.BP_ArcheryGamemode_C|GetTurnManager _gamemodereference))
  (bind _playerturn (Variables|/Game/Blueprints/ArcheryMinigameBlueprints/BP_ATurnManager.BP_ATurnManager_C|GetPlayerTurn _turnmanager))
  (bind _isassignedtarget (CallFunction|CheckAssignedTarget ArrowHit))
  (if _isassignedtarget
    (Class|BasePointCounter|AddPoints (Class|MinigameBase|GetPointCounter (Variables|Default|GetGameModeReference)) (Variables|/Game/Blueprints/ArcheryMinigameBlueprints/BP_ArcheryPlayer.BP_ArcheryPlayer_C|GetThisPlayerNum (Variables|/Game/Blueprints/ArcheryMinigameBlueprints/BP_AArrow.BP_AArrow_C|GetPlayer ArrowHit)) Points)
    (Default|CallSetScoreUI (Variables|Default|GetGameModeReference) _playerturn)
    (Default|CallScoreBounceUI (Variables|Default|GetGameModeReference) _playerturn)
    (CallFunction|PlayFeedback)
    (if (<= (Variables|/Game/Blueprints/ArcheryMinigameBlueprints/BP_ArcheryPlayer.BP_ArcheryPlayer_C|GetArrows (Variables|/Game/Blueprints/ArcheryMinigameBlueprints/BP_AArrow.BP_AArrow_C|GetPlayer ArrowHit)) 0)
      (Default|SetLastArrow ArrowHit)
      (Default|ArrowCleanuponHit ArrowHit ArrowLocationOnHit)
      (return Points)
      (else
        (return Points)))))

(fn CalculateDistancefromCenter
  (params (Arrow :type BP%20A%20Arrow%20Object%20Reference))
  (bind _collider (Variables|/Game/Blueprints/ArcheryMinigameBlueprints/BP_AArrow.BP_AArrow_C|GetCollider Arrow))
  (bind _returnvalue (Transformation|GetWorldLocation _collider))
  (return _returnvalue (Math|Vector|Distance(Vector) (Transformation|GetWorldLocation (Variables|Default|GetTestRingCollision)) _returnvalue)))

(fn CheckAssignedTarget
  (params (Arrow :type BP%20A%20Arrow%20Object%20Reference))
  (if (== (Variables|/Game/Blueprints/ArcheryMinigameBlueprints/BP_ArcheryPlayer.BP_ArcheryPlayer_C|GetAssignedTarget (Variables|/Game/Blueprints/ArcheryMinigameBlueprints/BP_AArrow.BP_AArrow_C|GetPlayer Arrow)) self)
    _
    (elif (Variables|/Script/MinigameCore.MinigameBase|GetbIsPractice (Variables|Default|GetGameModeReference))
      _
      (else
        (return false))))
  (return true))

(fn HighlightRing
  (params (FadeIn :type Boolean))
  (bind _highlightmat (Variables|Default|GetHighlightMat))
  (bind _highlightmat_2 (Variables|Default|GetHighlightMat))
  (if FadeIn
    ;[0.15 0.15 0.15 0.5] FadeIn
    (bind _returnvalue (Rendering|Material|GetScalarParameterValue _highlightmat_2 "OpacityVal" :!class /Script/Engine.MaterialInstanceDynamic))
    (Rendering|Material|SetScalarParameterValue _highlightmat_2 "OpacityVal" (+ _returnvalue 0.1) :!class /Script/Engine.MaterialInstanceDynamic)
    (else
      ;[0.15 0.15 0.15 0.5] FadeIn
      (bind _returnvalue_2 (Rendering|Material|GetScalarParameterValue _highlightmat "OpacityVal" :!class /Script/Engine.MaterialInstanceDynamic))
      (Rendering|Material|SetScalarParameterValue _highlightmat "OpacityVal" (- _returnvalue_2 0.1) :!class /Script/Engine.MaterialInstanceDynamic))))

(fn CalculateHighlightScale
  (params (Points :type Integer))
  (bind _highlight (Variables|Default|GetHighlight))
  (bind _returnvalue (Transformation|GetWorldScale _highlight))
  (bind _z (Math|Vector|BreakVector _returnvalue))
  (switch int Points
    (:Default
      (return) ; Should theoretically never be called
    )
    (:0
      (return) ; Should theoretically never be called
    )
    (:1
      (LocalVariables|SetNewScale (Math|Vector|MakeVector 2.5 2.5 _z)))
    (:2
      (LocalVariables|SetNewScale (Math|Vector|MakeVector 1.8 1.8 _z)))
    (:3
      (LocalVariables|SetNewScale (Math|Vector|MakeVector 1.0 1.0 _z)))
    (:4
      (LocalVariables|SetNewScale (Math|Vector|MakeVector 0.4 0.4 _z))))
  (Transformation|SetWorldScale3D (Variables|Default|GetHighlight) (LocalVariables|GetNewScale)))