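; BP_ATarget is a ring of an archery minigame target that handles arrow hits and scoring.
; On hit it stops the arrow, checks that the parent target is the shooter's assigned one (or practice mode is on), then adds a point, updates score UI, plays feedback and cleans up the arrow.
; Every arrow hit bounces the parent target.
; BeginPlay sets ring material from the Even flag and caches the game mode.
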(event EventBeginPlay
  (CallFunction|InitValues)
  (Variables|Default|SetOldPos (Transformation|GetActorLocation)))

(event Collision|EventHit
  (params (MyComp :type Primitive%20Component%20Object%20Reference) (Other :type Actor%20Object%20Reference) (OtherComp :type Primitive%20Component%20Object%20Reference) (bSelfMoved :type Boolean) (HitLocation :type Vector :default "0, 0, 0") (HitNormal :type Vector :default "0, 0, 0") (NormalImpulse :type Vector :default "0, 0, 0") (Hit :type Hit%20Result%20Structure%20%28by%20ref%29))
  (if (== (Utilities|GetClass Other) "/Game/Blueprints/ArcheryMinigameBlueprints/BP_AArrow.BP_AArrow_C")
    (bind _asbp_aarrow (Utilities|Casting|CastToBP_AArrow Other))
    (Variables|/Game/Blueprints/ArcheryMinigameBlueprints/BP_AArrow.BP_AArrow_C|SetInMotion _asbp_aarrow false)
    (Variables|/Game/Blueprints/ArcheryMinigameBlueprints/BP_AArrow.BP_AArrow_C|SetHitTarget _asbp_aarrow true)
    (CallFunction|AddPointsonTargetHit _asbp_aarrow HitLocation)
    (Default|EventTargetBounce (Variables|Default|GetTargetParent))
    (elif (== (Utilities|GetClass Other) "BP_ATarget_C") ; Check if colliding w/another ring\n\nCOLLISION ONLY HAPPENS DURING MOVEMENT from arrow hit
      (Collision|IgnoreActorwhenMoving (Variables|Default|GetCollider) Other false))))

(event Collision|EventActorBeginOverlap
  (params (OtherActor :type Actor%20Object%20Reference)))

(fn ConstructionScript)

(fn ChangeRingColor
  (if (Variables|Default|GetEven)
    (Rendering|Material|SetMaterial (Variables|Default|GetTargetRing) 0 (Variables|Default|GetRingMat))
    (else
      (Rendering|Material|SetMaterial (Variables|Default|GetTargetRing) 0 "/Engine/MaterialTemplates/VertexAnimation/AdvancedFlag.AdvancedFlag"))))

(fn AddPointsonTargetHit
  (params (self2 :type BP%20A%20Arrow%20Object%20Reference) (HitLocation :type Vector))
  (if (Actor|ActorHasTag self2 "ArrowParent") ; Check if the collision is with an arrow
    (bind _isassignedtarget (CallFunction|CheckAssignedTarget self2))
    (if _isassignedtarget ; Check if this is the assigned target
      (bind _outactors (Actor|GetAllActorsOfClass "/Game/Blueprints/ArcheryMinigameBlueprints/BP_ArcheryGamemode.BP_ArcheryGamemode_C"))
      (bind _output_get (Variables|Default|SetGameModeReference (Utilities|Array|Get(acopy) _outactors)))
      (Class|BasePointCounter|AddPoints (Class|MinigameBase|GetPointCounter _output_get) 0 1)
      (Default|CallSetScoreUI (Variables|Default|GetGameModeReference))
      (Default|CallScoreBounceUI (Variables|Default|GetGameModeReference) (Variables|/Game/Blueprints/ArcheryMinigameBlueprints/BP_ATurnManager.BP_ATurnManager_C|GetPlayerTurn (Variables|/Game/Blueprints/ArcheryMinigameBlueprints/BP_ArcheryGamemode.BP_ArcheryGamemode_C|GetTurnManager (Variables|Default|GetGameModeReference))))
      (Default|PlayFeedback (Variables|Default|GetTargetParent))
      (Default|ArrowCleanuponHit self2 self HitLocation))))

(fn InitValues
  (CallFunction|ChangeRingColor)
  (bind _returnvalue (Actor|GetActorOfClass "/Game/Blueprints/ArcheryMinigameBlueprints/BP_ArcheryGamemode.BP_ArcheryGamemode_C"))
  (Variables|Default|SetGameModeReference _returnvalue))

(fn CheckPrevPos
  (if (not (Utilities|Operators|EqualEqual (Transformation|GetActorLocation) (Variables|Default|GetOldPos) 0.0)) ; Shows change in position, change does only occur once!
    (Variables|Default|SetOldPos (Transformation|GetWorldLocation (Variables|Default|GetTargetRing))) ; Set old position to this position
  ))

(fn CheckAssignedTarget
  (params (Arrow :type BP%20A%20Arrow%20Object%20Reference))
  (if (== (Variables|/Game/Blueprints/ArcheryMinigameBlueprints/BP_ArcheryPlayer.BP_ArcheryPlayer_C|GetAssignedTarget (Variables|/Game/Blueprints/ArcheryMinigameBlueprints/BP_AArrow.BP_AArrow_C|GetPlayer Arrow)) (Variables|Default|GetTargetParent))
    _
    (elif (Variables|/Script/MinigameCore.MinigameBase|GetbIsPractice (Variables|Default|GetGameModeReference))
      _
      (else
        (return false))))
  (return true))