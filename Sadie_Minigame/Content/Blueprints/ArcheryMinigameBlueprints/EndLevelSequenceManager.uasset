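; Manager for the archery minigame's end-of-game cutscene, which picks a Level Sequence by winning player.
; On initialization it swaps the sequence, with an invalid winner falling through to EndP4, then destroys all player actors.
; It then caches gamemode UI and winner text, flags the TurnManager as in-cutscene, and hides the capture camera.
; After a fixed delay it ends the cutscene, clears the flag and calls the parent initializer.
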(event EventInitializeLevelSequence
  (params (SequenceActor :type Level%20Sequence%20Actor%20Object%20Reference))
  (bind _returnvalue (Class|MinigameCutsceneManager|GetWorld))
  (bind _returnvalue_2 (Class|MinigameCutsceneManager|GetWorld))
  (bind _asbp_archery_gamemode (Utilities|Casting|CastToBP_ArcheryGamemode (Variables|Default|GetCurrentMinigame)))
  ;[0.15 0.15 0.15 0.5] Change sequence based on player that won
  (CallFunction|SwitchCutsceneforWinner SequenceActor _asbp_archery_gamemode)
  (CallFunction|DestroyPlayers?) ; This actually makes the end cutscene play!!!!!!\nHowever it does destroy the players which defeats the purpose of the cutscene
  (Development|PrintString _returnvalue_2 (Utilities|GetDisplayName (Class|LevelSequencePlayer|GetActiveCameraComponent (Variables|/Script/LevelSequence.LevelSequenceActor|GetSequencePlayer SequenceActor))) true true "(R=0.008545,G=0.004311,B=1.000000,A=1.000000)")
  (Utilities|FlowControl|Delay _returnvalue_2 0.01)
  (CallFunction|InitValues)
  (Utilities|FlowControl|Delay _returnvalue 3.0) ; Wait for sequence to play
  (Development|PrintString _returnvalue "--PRE END CUTSCENE--") ; crash checking
  (Class|MinigameCutsceneManager|EndCutscene)
  (Default|ChangeCutsceneStatus (Variables|/Game/Blueprints/ArcheryMinigameBlueprints/BP_ArcheryGamemode.BP_ArcheryGamemode_C|GetTurnManager (Variables|Default|GetGameMode)) false)
  (Development|PrintString 0 "END CUTSCENE OVER") ; crash checking
  (|CallParentFunction SequenceActor))

(fn SetCutsceneText
  (params (UIText :type String) (ShouldFadeOut :type Boolean))
  (if ShouldFadeOut
    (UserInterface|Animation|PlayAnimation (Variables|Default|GetTurnUI) (Variables|/Game/Blueprints/ArcheryMinigameBlueprints/UI/BP_ArcheryUI.BP_ArcheryUI_C|GetFadeOut (Variables|Default|GetTurnUI)) 0.0 1 "Forward" 1.0 false)
    (else
      (Variables|/Script/UMG.TextBlock|SetText (Variables|/Game/Blueprints/ArcheryMinigameBlueprints/UI/BP_ArcheryUI.BP_ArcheryUI_C|GetPlayerTurnID (Variables|Default|GetTurnUI)) (Utilities|Text|ToText(String) UIText))
      (UserInterface|Animation|PlayAnimation (Variables|Default|GetTurnUI) (Variables|/Game/Blueprints/ArcheryMinigameBlueprints/UI/BP_ArcheryUI.BP_ArcheryUI_C|GetFadeIn (Variables|Default|GetTurnUI)) 0.0 1 "Forward" 1.0 false))))

(fn InitValues
  (bind _asbp_archery_gamemode (Utilities|Casting|CastToBP_ArcheryGamemode (Variables|Default|GetCurrentMinigame)))
  (bind _output_get (Variables|Default|SetGameMode _asbp_archery_gamemode))
  (Variables|Default|SetTurnUI (Variables|/Game/Blueprints/ArcheryMinigameBlueprints/BP_ArcheryGamemode.BP_ArcheryGamemode_C|GetPlayerScoreUI _output_get))
  (Variables|Default|SetUIWinnerStatement (Variables|/Game/Blueprints/ArcheryMinigameBlueprints/BP_ArcheryGamemode.BP_ArcheryGamemode_C|GetWinnerStatementToPass _output_get))
  (Variables|/Game/Blueprints/ArcheryMinigameBlueprints/BP_ATurnManager.BP_ATurnManager_C|SetinCutscene (Variables|/Game/Blueprints/ArcheryMinigameBlueprints/BP_ArcheryGamemode.BP_ArcheryGamemode_C|GetTurnManager (Variables|Default|GetGameMode)) true)
  (bind _returnvalue (Actor|GetActorOfClass (Class|MinigameCutsceneManager|GetWorld) "/MinigameCore/Game/BP_MinigameCapture.BP_MinigameCapture_C"))
  (bind _output_get_2 (Variables|Default|SetGameCam _returnvalue))
  (Rendering|SetActorHiddenInGame (Variables|Default|GetGameCam) true))

(fn SwitchCutsceneforWinner
  (params (LevelSequenceRef :type Level%20Sequence%20Actor%20Object%20Reference) (GameModeRef :type BP%20Archery%20Gamemode%20Object%20Reference))
  (bind _winner (Variables|/Game/Blueprints/ArcheryMinigameBlueprints/BP_ArcheryGamemode.BP_ArcheryGamemode_C|GetWinner GameModeRef))
  (Utilities|IsValid _winner ; Check for single winner or tie
    (:Is%20Valid
      (Development|PrintString (Class|MinigameCutsceneManager|GetWorld) (Utilities|GetDisplayName (Class|LevelSequenceActor|GetSequence LevelSequenceRef)) true true "(R=0.000000,G=0.000000,B=0.000000,A=1.000000)" 2e+01)
      (switch int (Variables|/Game/Blueprints/ArcheryMinigameBlueprints/BP_ArcheryPlayer.BP_ArcheryPlayer_C|GetThisPlayerNum _winner) ; Access none error, but still works
        (:Default
          (Variables|Default|SetWinnerLS "/Game/Sequences/TestNoCut.TestNoCut") ; In the event of a tie, default animation
        )
        (:0
          (Variables|Default|SetWinnerLS "/Game/Sequences/TestNoCut.TestNoCut"))
        (:1
          (Variables|Default|SetWinnerLS "/Game/Sequences/EndP2.EndP2"))
        (:2
          (Variables|Default|SetWinnerLS "/Game/Sequences/EndP3.EndP3"))
        (:3
          (Variables|Default|SetWinnerLS "/Game/Sequences/EndP4.EndP4" :!label _label))))
    (:Is%20Not%20Valid
      (goto _label)))
  (Class|LevelSequenceActor|SetSequence LevelSequenceRef (Variables|Default|GetWinnerLS))
  (Development|PrintString 0 (Utilities|GetDisplayName (Variables|Default|GetWinnerLS)) true true "(R=1.000000,G=0.403433,B=0.820796,A=1.000000)" 2e+01))

(fn DestroyPlayers?
  (bind _returnvalue (Actor|GetActorOfClass (Class|MinigameCutsceneManager|GetWorld) "/Game/Blueprints/ArcheryMinigameBlueprints/BP_ArcheryGamemode.BP_ArcheryGamemode_C"))
  (for _array_element (Variables|/Game/Blueprints/ArcheryMinigameBlueprints/BP_ArcheryGamemode.BP_ArcheryGamemode_C|GetPlayers _returnvalue)
    (Actor|DestroyActor _array_element)))