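; Game mode for the turn-based archery minigame, handling setup, reset, scoring feedback and winner selection.
; On start it gathers players and the turn manager, builds and shares the score UI, randomizes wind and places the capture actor over the shoulder.
; Reset restores turns and arrow counts after a delay for in-flight hits, then destroys arrows.
; Winners come from point-counter team totals outside practice mode, with ties supported.
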(event Custom|OnGameReset_Event
  (Utilities|FlowControl|Delay 2.0) ; Delay deleting arrows to allow shot arrows to hit targets and assign points
  (CallFunction|ResetArcheryGame) ; Is this necessary?
  (CallFunction|DeleteArrows))

(event EventOnMinigameEnd
  (Development|PrintString "START END GAME" true true "(R=0.436065,G=1.000000,B=0.000000,A=1.000000)")
  (Variables|/Game/Blueprints/ArcheryMinigameBlueprints/BP_ATurnManager.BP_ATurnManager_C|SetMoving (Variables|Default|GetTurnManager) false))

(event EventOnMinigameStart
  (bind _turnmanager (Variables|Default|GetTurnManager))
  (bind _players (Variables|Default|GetPlayers))
  (bind _playerturn (Variables|/Game/Blueprints/ArcheryMinigameBlueprints/BP_ATurnManager.BP_ATurnManager_C|GetPlayerTurn _turnmanager))
  (bind _output (Utilities|Array|Get(acopy) _players _playerturn))
  (CallFunction|CleanupPracticeMode)
  (CallFunction|InitValuesGamemode)
  (bind _cameraendpos (Default|OverlookShoulder (Variables|Default|GetTurnManager)))
  (bind _returnvalue (Actor|GetActorOfClass "/MinigameCore/Game/BP_MinigameCapture.BP_MinigameCapture_C"))
  (Transformation|SetActorLocation _returnvalue _cameraendpos false false)
  (Development|PrintString (Utilities|String|ToString(Integer) _playerturn) true true "(R=0.016977,G=1.000000,B=0.000000,A=1.000000)")
  (Default|CallSetNumArrowsUI _playerturn (Variables|/Game/Blueprints/ArcheryMinigameBlueprints/BP_ArcheryPlayer.BP_ArcheryPlayer_C|GetArrows _output) (Variables|/Game/Blueprints/ArcheryMinigameBlueprints/BP_ArcheryPlayer.BP_ArcheryPlayer_C|GetUIColor _output))
  (Default|CallIntroUI))

(fn ConstructionScript
  (|CallParentFunction))

(fn ResetArcheryGame
  (Variables|/Game/Blueprints/ArcheryMinigameBlueprints/BP_ATurnManager.BP_ATurnManager_C|SetPlayerTurn (Variables|Default|GetTurnManager) 0)
  (for (_ _array_index) (Variables|Default|GetPlayers)
    (Variables|/Game/Blueprints/ArcheryMinigameBlueprints/BP_ArcheryPlayer.BP_ArcheryPlayer_C|SetArrows (Utilities|Array|Get(acopy) (Variables|Default|GetPlayers) _array_index) 3)))

(fn InitValuesGamemode
  (bind _returnvalue (Actor|GetActorOfClass "/Game/Blueprints/ArcheryMinigameBlueprints/BP_ATurnManager.BP_ATurnManager_C"))
  (Variables|Default|SetTurnManager _returnvalue)
  (bind _outactors (Actor|GetAllActorsOfClass "/Game/Blueprints/ArcheryMinigameBlueprints/BP_ArcheryPlayer.BP_ArcheryPlayer_C"))
  ;[0.15 0 0] Get rid of!
  (bind _output_get (Variables|Default|SetPlayers _outactors))
  (Default|CleanUpPlayerArray (Variables|Default|GetTurnManager))
  (Development|PrintString (Utilities|String|ToString(Integer) (Utilities|Array|Length (Variables|/Game/Blueprints/ArcheryMinigameBlueprints/BP_ATurnManager.BP_ATurnManager_C|GetPlayersTurnManager (Variables|Default|GetTurnManager)))) true true "(R=1.000000,G=0.394040,B=0.525026,A=1.000000)")
  (bind _asbp_archery_ui (Utilities|Casting|CastToBP_ArcheryUIClass (Variables|Default|GetMinigameUIClass)))
  (bind _returnvalue_2 (Game|ConstructObjectfromClass _asbp_archery_ui))
  (Variables|Default|SetPlayerScoreUI _returnvalue_2)
  (Utilities|Array|Resize (Variables|Default|GetPlayerScoreTextBlocks) 4)
  (for (_array_element _array_index) (Variables|Default|GetPlayerScoreTextBlocks)
    (if (< _array_index (Utilities|Array|Length (Variables|Default|GetPlayers)))
      (bind _astext (Utilities|Casting|CastToTextBlock _array_element))
      (Variables|/Script/UMG.TextBlock|SetText _astext (Utilities|Text|MakeLiteralText (Utilities|Text|ToText(String) (Utilities|String|Append (Utilities|String|MakeLiteralString "Player ") (Utilities|String|ToString(Integer) (+ _array_index 1)) " Points: 0"))))
      (Default|RandomizeWindDirection (Utilities|Array|Get(acopy) (Variables|Default|GetPlayers) (Variables|/Game/Blueprints/ArcheryMinigameBlueprints/BP_ATurnManager.BP_ATurnManager_C|GetPlayerTurn (Variables|Default|GetTurnManager))))))
  (CallFunction|AssignAllUIVariables)
  (Default|CallSetScoreUI))

(fn DeleteArrows
  (bind _outactors (Actor|GetAllActorsOfClass "/Game/Blueprints/ArcheryMinigameBlueprints/BP_AArrow.BP_AArrow_C"))
  (LocalVariables|SetArrows _outactors)
  (for _array_element (LocalVariables|GetArrows) ; Delete arrows, may need to delay in loading state?
    (Actor|DestroyActor _array_element)))

(fn CalculateWinner
  (bind _winners (Variables|Default|GetWinners))
  (bind _winners_2 (Variables|Default|GetWinners))
  (if (not (Variables|Default|GetbIsPractice)) ; Ensure a winner is not set in practice mode
    (for (_array_element _array_index) (Variables|/Script/MinigameCore.BasePointCounter|GetTeamPoints (Variables|Default|GetBasePointCounter))
      (if (> _array_element (LocalVariables|GetTopScore)) ; If greater than, set new high score.  Need to account for ties as well
        (LocalVariables|SetTopScore _array_element)
        (Utilities|Array|Clear _winners_2)
        (Utilities|Array|Add _winners_2 (Utilities|Array|Get(acopy) (Variables|Default|GetPlayers) _array_index))
        (if (> (Utilities|Array|Length _winners) 1) :!label _label
          (Variables|Default|SetWinner 0) ; Set winner to null if tie
          (else
            (Variables|Default|SetWinner (Utilities|Array|Get(acopy) _winners)) ; Only one winner
          ))
        (elif (== _array_element (LocalVariables|GetTopScore)) ; Potential tie
          (Utilities|Array|Add (Variables|Default|GetWinners) (Utilities|Array|Get(acopy) (Variables|Default|GetPlayers) _array_index))
          (goto _label))))
    (for _array_element_2 (Variables|Default|GetWinners)
      (LocalVariables|SetWinnerStatement (Utilities|String|Append (LocalVariables|GetWinnerStatement) "Player " (Utilities|String|ToString(Integer) (+ (Variables|/Game/Blueprints/ArcheryMinigameBlueprints/BP_ArcheryPlayer.BP_ArcheryPlayer_C|GetThisPlayerNum _array_element_2) 1)))))
    (Development|PrintString (LocalVariables|GetWinnerStatement) true true "(R=1.000000,G=0.000000,B=0.235128,A=1.000000)" 4e+01)
    (return (Utilities|Array|Length (Variables|Default|GetWinners)) (LocalVariables|GetWinnerStatement))))

(fn CleanupPracticeMode
  (Utilities|Array|Clear (Variables|Default|GetPlayers))
  (if (not (Variables|Default|GetbIsPractice))
    (bind _returnvalue (Actor|GetActorOfClass "/Game/Blueprints/ArcheryMinigameBlueprints/BP_ATurnManager.BP_ATurnManager_C"))
    (Utilities|Array|Clear (Variables|/Game/Blueprints/ArcheryMinigameBlueprints/BP_ATurnManager.BP_ATurnManager_C|GetPlayersTurnManager _returnvalue))))

(fn PlayScoreAnim
  (params (PlayerID :type Integer))
  (bind _playerscoreui (Variables|Default|GetPlayerScoreUI))
  (switch int PlayerID
    (:0
      (UserInterface|Animation|PlayAnimation _playerscoreui (Variables|/Game/Blueprints/ArcheryMinigameBlueprints/UI/BP_ArcheryUI.BP_ArcheryUI_C|GetBounce1 _playerscoreui) 0.0 1 "Forward" 1.0 false))
    (:1
      (UserInterface|Animation|PlayAnimation _playerscoreui (Variables|/Game/Blueprints/ArcheryMinigameBlueprints/UI/BP_ArcheryUI.BP_ArcheryUI_C|GetBounce2 _playerscoreui) 0.0 1 "Forward" 1.0 false))
    (:2
      (UserInterface|Animation|PlayAnimation _playerscoreui (Variables|/Game/Blueprints/ArcheryMinigameBlueprints/UI/BP_ArcheryUI.BP_ArcheryUI_C|GetBounce3 _playerscoreui) 0.0 1 "Forward" 1.0 false))
    (:3
      (UserInterface|Animation|PlayAnimation _playerscoreui (Variables|/Game/Blueprints/ArcheryMinigameBlueprints/UI/BP_ArcheryUI.BP_ArcheryUI_C|GetBounce4 _playerscoreui) 0.0 1 "Forward" 1.0 false))))

(fn AssignAllUIVariables
  (for _array_element (Variables|Default|GetPlayers)
    (Variables|/Game/Blueprints/ArcheryMinigameBlueprints/BP_ArcheryPlayer.BP_ArcheryPlayer_C|SetWindUI _array_element (Variables|Default|GetPlayerScoreUI)))
  (Variables|/Game/Blueprints/ArcheryMinigameBlueprints/BP_ATurnManager.BP_ATurnManager_C|SetPlayerTurnUI (Variables|Default|GetTurnManager) (Variables|Default|GetPlayerScoreUI)))