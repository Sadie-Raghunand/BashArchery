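; BP_Elevator is a tutorial elevator actor that starts moving its Cube on BeginPlay, with no player trigger.
; The Move timeline's Track drives a lerp between the TopPosition and BottomPosition world locations and is printed each update.
; On Finished, MoveElevator reverses the timeline for the return trip; nothing calls Play again, so it makes no repeating round trip.
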(event Custom|MoveElevator
  (bind _track (Timeline|Move Reverse)
    (:Update
      (Development|PrintString (Utilities|String|ToString(Float) _track))
      (Transformation|SetWorldLocation (Variables|Default|GetCube) (Math|Vector|Lerp(Vector) (Transformation|GetWorldLocation (Variables|Default|GetTopPosition)) (Transformation|GetWorldLocation (Variables|Default|GetBottomPosition)) _track) false false))
    (:Finished
      (CallFunction|MoveElevator))))

(event EventBeginPlay
  (bind _track (Timeline|Move Play)
    (:Update
      (Development|PrintString (Utilities|String|ToString(Float) _track))
      (Transformation|SetWorldLocation (Variables|Default|GetCube) (Math|Vector|Lerp(Vector) (Transformation|GetWorldLocation (Variables|Default|GetTopPosition)) (Transformation|GetWorldLocation (Variables|Default|GetBottomPosition)) _track) false false))
    (:Finished
      (CallFunction|MoveElevator))))

(event Collision|EventActorBeginOverlap
  (params (OtherActor :type Actor%20Object%20Reference)))

(event EventTick
  (params (DeltaSeconds :type Float%20%28single-precision%29)))

(fn ConstructionScript)