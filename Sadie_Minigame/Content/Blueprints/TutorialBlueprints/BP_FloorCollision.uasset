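; BP_FloorCollision is a tutorial actor that responds to a CollectPickup event by counting pickups and recoloring its Cube.
; The event runs a sequence: it increments PickupsCollected and prints the total, then sets the Cube's first material slot to the red AnimSharingRed material.
; BeginPlay, overlap and Tick are unused, so the actor does no collision detection itself and relies on CollectPickup being triggered.
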(event EventBeginPlay)

(event Collision|EventActorBeginOverlap
  (params (OtherActor :type Actor%20Object%20Reference)))

(event EventTick
  (params (DeltaSeconds :type Float%20%28single-precision%29)))

(event Custom|CollectPickup
  (Utilities|FlowControl|Sequence
    (:then_0
      (CallFunction|IncrememntPickups))
    (:then_1
      (CallFunction|SetBoxMaterial))))

(fn ConstructionScript)

(fn IncrememntPickups
  (bind _output_get (Variables|Default|SetPickupsCollected (+ (Variables|Default|GetPickupsCollected) 1)))
  (Development|PrintString (Utilities|String|ToString(Integer) _output_get)))

(fn SetBoxMaterial
  (Rendering|Material|SetMaterial (Variables|Default|GetCube) 0 "/AnimationSharing/AnimSharingRed.AnimSharingRed"))