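; Turn manager for the archery minigame that steps through players and moves the capture camera to each one.
; ChangePlayerTurn increments the turn and flags movement, so Tick plays a timeline that lerps itself and the camera toward that player, rotating toward their target.
; Once turns exceed the player list, it fires the gamemode's reset event.
; Work in progress: player gathering is disconnected, CheckInPosition is never called here, and debug prints remain.
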(event EventBeginPlay
  (CallFunction|InitValues)
  (CallFunction|MoveCameratoNextPos (stale EventTick _newtrack_0)))

(event EventTick
  (params (DeltaSeconds :type Float%20%28single-precision%29))
  (if (Variables|Default|GetMoving)
    (bind _newtrack_0 (Timeline|MoveCamera Play) ; Move camera to the side to position in front of next player's target
      (:Update
        (if (< (Variables|Default|GetPlayerTurn) (Utilities|Array|Length (Variables|Default|GetPlayers))) ; Check to see if there are any more players' whose turn it will be
          (CallFunction|MoveCameratoNextPos _newtrack_0)
          (else
            (CallFunction|ResetThisGame)))))))

(fn ConstructionScript)

(fn ChangePlayerTurn
  (if (not (>= (Variables|Default|GetPlayerTurn) 4)) ; If true, end minigame, if false, move to next player
    (Math|Integer|IncrementInt (Variables|Default|GetPlayerTurn)
      (:%20%20
        (Variables|Default|SetMoving true)
        (Variables|Default|SetInPos false)))))

(fn InitValues
  (Variables|Default|SetTurnsTotal 0) ; Need to get accurate num players after all players are added externally
  (bind _returnvalue (Actor|GetActorOfClass "/MinigameCore/BP_MinigameCapture.BP_MinigameCapture_C"))
  (Variables|Default|SetCamera _returnvalue)
  (bind _returnvalue_2 (Actor|GetActorOfClass "/Game/Blueprints/MinigameBlueprints/BP_ArcheryGamemode.BP_ArcheryGamemode_C"))
  (Variables|Default|SetGameMode _returnvalue_2))

(fn MoveCameratoNextPos
  (params (Alpha :type Float%20%28single-precision%29))
  (bind _returnvalue (Transformation|GetActorLocation))
  (bind _players (Variables|Default|GetPlayers))
  (bind _playerturn (Variables|Default|GetPlayerTurn))
  (bind _output (Utilities|Array|Get(acopy) _players _playerturn))
  (bind _returnvalue_2 (Transformation|GetActorLocation _output))
  (bind _returnvalue_3 (Math|Vector|Lerp(Vector) _returnvalue _returnvalue_2 Alpha))
  (Transformation|SetWorldLocation (Variables|Default|GetDefaultSceneRoot) _returnvalue_3 false false)
  (Transformation|SetWorldLocation (Variables|/Script/Engine.Actor|GetRootComponent (Variables|Default|GetCamera)) _returnvalue_3 false false) ; Error - accessed non trung to acces index 1
  (if (not (Variables|Default|GetInPos)) ; Check if in position
    (Transformation|SetActorRotation (Variables|Default|GetCamera) (Math|Rotator|FindLookatRotation (Math|Rotator|GetRotationXVector (Transformation|GetActorRotation (Variables|Default|GetCamera))) (Transformation|GetActorLocation (Utilities|Array|Get(acopy) (Variables|Default|GetTargets) (Variables|Default|GetPlayerTurn)))))
    (Variables|Default|SetMoving false)
    (Development|PrintString "Cam NOT in pos" true true "(R=0.000000,G=0.660000,B=1.000000,A=1.000000)" 0.5)))

(fn ResetThisGame
  (Default|OnGameResetEvent (Variables|Default|GetGameMode)) ; Set camera position back to begining position
  (Variables|Default|SetMoving true))

(fn CheckinPosition
  (if (== (Transformation|GetActorTransform) (Transformation|GetActorTransform (Utilities|Array|Get(acopy) (Variables|Default|GetPlayers) (Variables|Default|GetPlayerTurn))))
    (Variables|Default|SetInPos true)))