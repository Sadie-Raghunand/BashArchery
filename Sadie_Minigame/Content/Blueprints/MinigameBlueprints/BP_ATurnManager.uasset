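; Turn manager for the archery minigame that moves the capture camera to an over-the-shoulder view of each player in turn.
; After a short spawn delay it hides unassigned targets and their rings, then plays a timeline, replayed from Tick while Moving.
; The timeline lerps the manager to the current player and snaps the camera to an offset with zero rotation.
; When no players remain, it fires the GameMode's reset event.
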(event EventBeginPlay
  (Utilities|FlowControl|Delay 0.5) ; Prevent move cam from happening before players are spawned in
  (CallFunction|InitValues)
  (bind _newtrack_0 (Timeline|MoveCamera Play) ; Move camera to the side to position in front of next player's target
    (:Update
      (if (< (Variables|Default|GetPlayerTurn) (Utilities|Array|Length (Variables|Default|GetPlayers))) ; Check to see if there are any more players' whose turn it will be
        (bind _cameraendpos (CallFunction|OverlookShoulder))
        (CallFunction|MoveCameratoNextPos _newtrack_0 _cameraendpos)
        (else
          (Development|PrintString "No more players, resetting game")
          (CallFunction|ResetThisGame))))))

(event EventTick
  (params (DeltaSeconds :type Float%20%28single-precision%29))
  (if (Variables|Default|GetMoving)
    (bind _newtrack_0 (Timeline|MoveCamera Play) ; Move camera to the side to position in front of next player's target
      (:Update
        (if (< (Variables|Default|GetPlayerTurn) (Utilities|Array|Length (Variables|Default|GetPlayers))) ; Check to see if there are any more players' whose turn it will be
          (bind _cameraendpos (CallFunction|OverlookShoulder))
          (CallFunction|MoveCameratoNextPos _newtrack_0 _cameraendpos)
          (else
            (Development|PrintString "No more players, resetting game")
            (CallFunction|ResetThisGame)))))))

(fn ConstructionScript)

(fn ChangePlayerTurn
  (Development|PrintString "Change player turn called")
  (if (not (>= (Variables|Default|GetPlayerTurn) 4)) ; f true, end minigame, if false, move to next player
    (bind _result (Math|Integer|IncrementInt (Variables|Default|GetPlayerTurn))
      (:%20%20
        (Variables|Default|SetPlayerTurn _result)
        (Variables|Default|SetMoving true)
        (Variables|Default|SetInPos false)))))

(fn InitValues
  (bind _returnvalue (Actor|GetActorOfClass "/MinigameCore/Game/BP_MinigameCapture.BP_MinigameCapture_C"))
  (Variables|Default|SetCamera _returnvalue)
  (bind _returnvalue_2 (Actor|GetActorOfClass "/Game/Blueprints/MinigameBlueprints/BP_ArcheryGamemode.BP_ArcheryGamemode_C"))
  (Variables|Default|SetGameMode _returnvalue_2)
  (bind _arrayindex (Utilities|Array|ReverseforEachLoop (Variables|Default|GetTargets)) ; Set targets not assigned to a player inactive
    (:LoopBody
      (if (not (> (Variables|Default|GetTurnsTotal) _arrayindex))
        (Rendering|SetActorHiddenInGame (Utilities|Array|Get(acopy) (Variables|Default|GetTargets) _arrayindex) true)
        (for _array_element (Variables|/Game/Blueprints/MinigameBlueprints/BP_ATargetParent.BP_ATargetParent_C|GetTargetRings (Utilities|Array|Get(acopy) (Variables|Default|GetTargets) _arrayindex)) ; Set rings inactive as well
          (Rendering|SetActorHiddenInGame _array_element true))
        (Transformation|SetActorRotation (Variables|Default|GetCamera))))))

(fn MoveCameratoNextPos
  (params (Alpha :type Float%20%28single-precision%29) (CameraPos :type Vector))
  (Transformation|SetWorldLocation (Variables|Default|GetDefaultSceneRoot) (Math|Vector|Lerp(Vector) (Transformation|GetActorLocation) (Transformation|GetActorLocation (Utilities|Array|Get(acopy) (Variables|Default|GetPlayers) (Variables|Default|GetPlayerTurn))) Alpha) false false) ; Set this position
  (Transformation|SetWorldLocation (Variables|/Script/Engine.Actor|GetRootComponent (Variables|Default|GetCamera)) CameraPos false false) ; Set camera position
  (Transformation|SetActorRotation (Variables|Default|GetCamera)) ; Force no rotation on camera
)

(fn ResetThisGame
  (Default|OnGameResetEvent (Variables|Default|GetGameMode)) ; Set camera position back to begining position
  (Variables|Default|SetMoving true))

(fn CheckinPosition
  (if (== (Transformation|GetActorTransform) (Transformation|GetActorTransform (Utilities|Array|Get(acopy) (Variables|Default|GetPlayers) (Variables|Default|GetPlayerTurn))))
    (Variables|Default|SetInPos true)))

(fn RotateTowardsTarget
  (Transformation|SetActorRotation (Variables|Default|GetCamera) (Math|Rotator|FindLookatRotation (Math|Rotator|GetRotationXVector (Transformation|GetActorRotation)) (Transformation|GetActorLocation (Utilities|Array|Get(acopy) (Variables|Default|GetTargets) (Variables|Default|GetPlayerTurn)))))
  (Variables|Default|SetMoving false)
  (Development|PrintString "Cam NOT in pos" true true "(R=0.000000,G=0.660000,B=1.000000,A=1.000000)" 0.5))

(fn OnEndMovement
  (Development|PrintString "IN POSITION"))

(fn OverlookShoulder
  (bind _players (Variables|Default|GetPlayers))
  (bind _playerturn (Variables|Default|GetPlayerTurn))
  (bind _output (Utilities|Array|Get(acopy) _players _playerturn))
  (bind _returnvalue (Transformation|GetActorLocation _output))
  (bind (_x _y _z) (Math|Vector|BreakVector _returnvalue))
  (return (Math|Vector|MakeVector (+ _x (LocalVariables|GetXOffset)) (+ _y (LocalVariables|GetYOffset)) (+ _z (LocalVariables|GetZOffset)))))