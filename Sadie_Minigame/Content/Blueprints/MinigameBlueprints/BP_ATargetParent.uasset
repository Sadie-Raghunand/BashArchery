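; Parent actor for a minigame target built from a set of ring actors, able to jump to random spots in the player lane.
; ParentRings attaches the rings to the root, then calls ChangeLocation.
; ChangeLocation moves the root within a box centered ahead of its start position, switching the ring colliders' constraint mode off around the move.
; A vertical hit-reaction lerp exists but is not wired to Tick.
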(event EventBeginPlay
  (Variables|Default|SetCenterPos (+ (Transformation|GetActorLocation) "1000.000000,0.000000,0.000000")))

(event EventTick
  (params (DeltaSeconds :type Float%20%28single-precision%29)))

(fn ConstructionScript)

(fn ChangeLocation
  (CallFunction|DisablePhysicsConstraints)
  (Transformation|SetWorldLocation (Variables|Default|GetDefaultSceneRoot) (Math|Random|RandomPointinBoundingBox (Variables|Default|GetCenterPos) "75.000000,200.000000,0.000000") false false) ; Change parent location
  (CallFunction|EnablePhysicsConstraints))

(fn ParentRings
  ;[1 1 1 1 12] Test changing each ring's location
  (for _array_element (Variables|Default|GetTargetRings)
    (Transformation|AttachComponentToComponent _array_element (Variables|Default|GetDefaultSceneRoot) "None" "SnapToTarget" "KeepRelative" "KeepRelative" true) ; Make target rings children of parent
  )
  (CallFunction|ChangeLocation) ; The actual location in the inspector shows a change in pos, but not visible in game?
)

(fn DisablePhysicsConstraints
  (for _array_element (Variables|Default|GetTargetRings)
    (Class|PrimitiveComponent|SetConstraintMode (Variables|/Game/Blueprints/MinigameBlueprints/BP_ATarget.BP_ATarget_C|GetCollider _array_element) "None")))

(fn EnablePhysicsConstraints
  (for _array_element (Variables|Default|GetTargetRings)
    (Class|PrimitiveComponent|SetConstraintMode (Variables|/Game/Blueprints/MinigameBlueprints/BP_ATarget.BP_ATarget_C|GetCollider _array_element) "Default")))

(fn ReacttoHit
  (params (InterpolateVal :type Float%20%28double-precision%29))
  (bind _returnvalue (Transformation|GetActorLocation))
  (bind _returnvalue_2 (Transformation|GetActorLocation))
  (bind (_x _y _z) (Math|Vector|BreakVector _returnvalue))
  (bind (_x_2 _y_2 _z_2) (Math|Vector|BreakVector _returnvalue_2))
  (if (>= (.Z (Math|Vector|BreakVector (Transformation|GetActorLocation))) (LocalVariables|GetPeakZ))
    (Transformation|SetActorLocation (Math|Vector|Lerp(Vector) (Transformation|GetActorLocation) (Math|Vector|MakeVector _x_2 _y_2 0.0) InterpolateVal) false false)
    (else
      (Transformation|SetActorLocation (Math|Vector|Lerp(Vector) (Transformation|GetActorLocation) (Math|Vector|MakeVector _x _y (+ _z 1.0)) InterpolateVal) false false))))