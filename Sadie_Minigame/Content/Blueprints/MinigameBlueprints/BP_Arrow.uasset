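; BP_Arrow is the arrow actor for an archery minigame, apparently work in progress.
; On BeginPlay it caches the player, capture camera and target, then plays a Multiplier-rated timeline that nudges it along world +X by lerped offsets, without sweeping.
; Tick draws a debug line from the arrow using the camera's forward vector.
; An impulse-based launch with player wind and a rotation-matching CalculateForce remain, but never run.
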(event EventBeginPlay
  (CallFunction|InitValues)
  (Components|Timeline|SetPlayRate (Variables|Default|GetTimeline) (Variables|Default|GetMultiplier))
  (bind _newtrack_0 (Timeline|Timeline Play)
    (:Update
      (CallFunction|LaunchArrowForward _newtrack_0))))

(event EventTick
  (params (DeltaSeconds :type Float%20%28single-precision%29))
  (Rendering|Debug|DrawDebugLine :LineStart (Transformation|GetActorLocation) :LineEnd (Transformation|GetActorForwardVector (Variables|Default|GetCamera)) :Thickness 1e+01))

(fn ConstructionScript)

(fn [NOTINUSE]LaunchArrow
  (params (Direction :type Vector))
  (bind _returnvalue (Transformation|GetActorForwardVector))
  (Rendering|Debug|DrawDebugLine :LineStart (Transformation|GetActorLocation (Variables|Default|GetCamera)) :LineEnd _returnvalue :Duration 1e+01 :Thickness 5.0)
  (bind _output_get (Variables|Default|SetForce _returnvalue))
  (Physics|AddImpulse (Variables|Default|GetArrowHead) (Math|Vector|MakeVector (.X (Class|KismetMathLibrary|BreakVector3f (Math|Vector|MakeVector (.X (Math|Vector|BreakVector (* _output_get (Variables|Default|GetMultiplier)))) (.Y (Math|Vector|BreakVector (* _output_get (Variables|Default|GetMultiplier)))) (.Z (Math|Vector|BreakVector (* _output_get (Variables|Default|GetMultiplier))))))) (+ (.Y (Class|KismetMathLibrary|BreakVector3f (Math|Vector|MakeVector (.X (Math|Vector|BreakVector (* _output_get (Variables|Default|GetMultiplier)))) (.Y (Math|Vector|BreakVector (* _output_get (Variables|Default|GetMultiplier)))) (.Z (Math|Vector|BreakVector (* _output_get (Variables|Default|GetMultiplier))))))) (Variables|/Game/Blueprints/MinigameBlueprints/BP_ArcheryPlayer.BP_ArcheryPlayer_C|GetWind (Variables|Default|GetPlayer))) (.Z (Class|KismetMathLibrary|BreakVector3f (Math|Vector|MakeVector (.X (Math|Vector|BreakVector (* _output_get (Variables|Default|GetMultiplier)))) (.Y (Math|Vector|BreakVector (* _output_get (Variables|Default|GetMultiplier)))) (.Z (Math|Vector|BreakVector (* _output_get (Variables|Default|GetMultiplier)))))))) "None" true))

(fn CalculateForce
  (Transformation|SetActorRotation (Transformation|GetActorRotation (Variables|Default|GetPlayer))) ; Quick note before I forget, ,maybe forgo the actor transfrm forward and switch to lerp forward for a duration dependent on the the force applied?
  (Development|PrintString (Utilities|String|ToString(Vector) (Transformation|GetActorForwardVector)) true true "(R=1.000000,G=0.041135,B=0.000000,A=1.000000)")
  (Development|PrintString (Utilities|String|ToString(Vector) (Transformation|GetActorForwardVector (Variables|Default|GetCamera)))))

(fn InitValues
  (bind _returnvalue (Actor|GetActorOfClass "/Game/Blueprints/MinigameBlueprints/BP_ArcheryPlayer.BP_ArcheryPlayer_C"))
  (Variables|Default|SetPlayer _returnvalue)
  (bind _returnvalue_2 (Actor|GetActorOfClass "/MinigameCore/BP_MinigameCapture.BP_MinigameCapture_C"))
  (Variables|Default|SetCamera _returnvalue_2)
  (bind _returnvalue_3 (Actor|GetActorOfClass "/Game/Blueprints/MinigameBlueprints/BP_TargetParent.BP_TargetParent_C"))
  (Variables|Default|SetTargetTestForward _returnvalue_3))

(fn LaunchArrowForward
  (params (Alpha :type Float%20%28single-precision%29))
  (Transformation|SetActorLocation (Math|Vector|Lerp(Vector) (Transformation|GetActorLocation) (+ (Transformation|GetActorLocation) "1.000000,0.000000,0.000000") Alpha) false false))