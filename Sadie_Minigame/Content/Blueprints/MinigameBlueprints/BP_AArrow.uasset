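; Arrow projectile for the archery minigame, which flies with player-set wind and destroys itself on floor impact or beyond a distance from the capture camera.
; A looping Timeline lerps it forward with wind drift, while Tick overrides physics velocity to fake an arc, rising then falling based on lifetime versus Multiplier.
; Arrow-to-arrow hits briefly disable collision.
; Destroying the last arrow passes the turn through BP_ATurnManager.
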(event OnComponentHit(Collider)
  (params (HitComponent :type Primitive%20Component%20Object%20Reference) (OtherActor :type Actor%20Object%20Reference) (OtherComp :type Primitive%20Component%20Object%20Reference) (NormalImpulse :type Vector :default "0, 0, 0") (Hit :type Hit%20Result%20Structure%20%28by%20ref%29))
  (if (Components|ComponentHasTag HitComponent "ArrowTag")
    (Collision|SetActorEnableCollision false) ; Prevent inital collision, realistically arrows would be thinner than the spheres, so collisions would happen less often and be more realistic
    (Utilities|FlowControl|Delay 0.2)
    (Collision|SetActorEnableCollision true)))

(event Custom|KeepMoving
  (bind _newtrack_0 (Timeline|Timeline PlayFromStart) ; Start moving once arrow is instantaited
    (:Update
      (Development|PrintString (Utilities|String|ToString(Float) _newtrack_0))
      (CallFunction|LaunchArrowForward 0.5))
    (:Finished
      (CallFunction|KeepMoving))))

(event EventBeginPlay
  (CallFunction|InitValues)
  (Components|Timeline|SetPlayRate (Variables|Default|GetTimeline) (Variables|Default|GetMultiplier))
  (bind _newtrack_0 (Timeline|Timeline Play) ; Start moving once arrow is instantaited
    (:Update
      (Development|PrintString (Utilities|String|ToString(Float) _newtrack_0))
      (CallFunction|LaunchArrowForward 0.5))
    (:Finished
      (CallFunction|KeepMoving))))

(event EventTick
  (params (DeltaSeconds :type Float%20%28single-precision%29))
  (bind _returnvalue (Transformation|GetVelocity))
  (bind (_x _y _z) (Math|Vector|BreakVector _returnvalue))
  (bind _velocityadditive (CallFunction|ApplyUpward/DownwardForce (Actor|GetGameTimeSinceCreation) (Variables|Default|GetMultiplier)))
  (bind _iszvalidafter (CallFunction|SetArrowVelocity _velocityadditive _y (> _z 0.0)))
  (if _iszvalidafter ; Prevent backwards movement when collions b/w arrows occur
    _
    (else
      _))
  (CallFunction|DestroyArrow false) ; Check distance from shooting position, destroy if too far
)

(event Collision|EventHit
  (params (MyComp :type Primitive%20Component%20Object%20Reference) (Other :type Actor%20Object%20Reference) (OtherComp :type Primitive%20Component%20Object%20Reference) (bSelfMoved :type Boolean) (HitLocation :type Vector :default "0, 0, 0") (HitNormal :type Vector :default "0, 0, 0") (NormalImpulse :type Vector :default "0, 0, 0") (Hit :type Hit%20Result%20Structure%20%28by%20ref%29))
  (if (Utilities|Enum|Equal(Enum) (Utilities|GetDisplayName Other) "Floor")
    (Development|PrintString "Hit the floor" true true "(R=1.000000,G=0.790707,B=0.000000,A=1.000000)")
    (CallFunction|DestroyArrow true)))

(fn ConstructionScript)

(fn InitValues
  (bind _returnvalue (Actor|GetActorOfClass "/Game/Blueprints/MinigameBlueprints/BP_ArcheryPlayer.BP_ArcheryPlayer_C")) ; Player
  (Variables|Default|SetPlayer _returnvalue)
  (bind _returnvalue_2 (Actor|GetActorOfClass "/MinigameCore/BP_MinigameCapture.BP_MinigameCapture_C")) ; Camera
  (Variables|Default|SetCamera _returnvalue_2)
  (bind _returnvalue_3 (Actor|GetActorOfClass "/Game/Blueprints/MinigameBlueprints/BP_ATargetParent.BP_ATargetParent_C")) ; Target parent
  (Variables|Default|SetTargetTestForward _returnvalue_3)
  (bind _returnvalue_4 (Actor|GetActorOfClass "/Game/Blueprints/MinigameBlueprints/BP_ATurnManager.BP_ATurnManager_C")) ; Turn manager
  (Variables|Default|SetTurnManager _returnvalue_4)
  (Transformation|SetActorRotation (Transformation|GetActorRotation (Variables|Default|GetPlayer))))

(fn LaunchArrowForward
  (params (Alpha :type Float%20%28single-precision%29))
  (Transformation|SetActorRelativeLocation (Math|Vector|Lerp(Vector) (Transformation|GetActorLocation) (+ (.Location (Math|Transform|BreakTransform (Transformation|GetRelativeTransform (Variables|Default|GetCollider)))) (Math|Vector|MakeVector (Variables|/Game/Blueprints/MinigameBlueprints/BP_ArcheryPlayer.BP_ArcheryPlayer_C|GetWind (Variables|Default|GetPlayer)) 1.0 0.0)) Alpha))
  (return (+ (.Location (Math|Transform|BreakTransform (Transformation|GetRelativeTransform (Variables|/Script/MinigameCore.MinigameCapture|GetSceneCapture (Variables|Default|GetCamera))))) "1.000000,0.000000,0.000000")))

(fn ApplyWind
  (Physics|AddForce :Force (Math|Vector|MakeVector (Variables|/Game/Blueprints/MinigameBlueprints/BP_ArcheryPlayer.BP_ArcheryPlayer_C|GetWind (Variables|Default|GetPlayer)) 0.0 0.0)))

(fn DestroyArrow
  (params (HitFloor :type Boolean))
  (if HitFloor ; Check if the floor wa hit, bypass distance requirement
    (if (Variables|Default|GetLastArrow) :!label _label ; Whether this is the last arrow this player has or not
      (Development|PrintString "About to change player vira arrow")
      (Default|ChangePlayerTurn (Variables|Default|GetTurnManager))
      (CallFunction|ArrowCleanup)
      (else
        (CallFunction|ArrowCleanup)))
    (elif (> (Transformation|GetDistanceTo (Variables|Default|GetCamera)) (Variables|Default|GetDestroyDistance)) ; Check if at destroy distance
      (goto _label))))

(fn SetLastArrow
  (Variables|Default|SetLastArrow true))

(fn ArrowCleanup
  (Variables|/Game/Blueprints/MinigameBlueprints/BP_ArcheryPlayer.BP_ArcheryPlayer_C|SetThisArrow (Variables|Default|GetPlayer) 0)
  (Actor|DestroyActor))

(fn ApplyUpward/DownwardForce
  (params (SecondsPassed :type Float%20%28double-precision%29) (StrengthOfFlex :type Float%20%28double-precision%29))
  (bind _returnvalue (Math|Vector|VectorDown))
  (bind _returnvalue_2 (Math|Vector|VectorUp))
  (bind _returnvalue_3 (* _returnvalue SecondsPassed))
  (bind _returnvalue_4 (/ _returnvalue_2 SecondsPassed))
  (bind _returnvalue_5 (* _returnvalue_4 "0.000000,0.000000,10.000000"))
  (bind _returnvalue_6 (* _returnvalue_3 "0.000000,0.000000,10.000000"))
  (if (> SecondsPassed (/ StrengthOfFlex 2.0)) ; If seconds pass is longer, start going down, if less then go up
    (Physics|SetPhysicsLinearVelocity (Variables|Default|GetCollider) _returnvalue_6 false "None") ; Downward movement
    (Physics|SetEnableGravity (Variables|Default|GetCollider) true)
    (LocalVariables|SetAddToVelocity _returnvalue_6)
    (else
      (Physics|SetPhysicsLinearVelocity (Variables|Default|GetCollider) _returnvalue_5 false "None") ; Upward movement
      (LocalVariables|SetAddToVelocity _returnvalue_5)))
  (return (LocalVariables|GetAddToVelocity)))

(fn SetArrowVelocity
  (params (VerticalVelocity :type Vector) (ZVelocity :type Float%20%28double-precision%29) (IsZValid :type Boolean))
  (if IsZValid
    (Physics|SetPhysicsLinearVelocity (Variables|Default|GetCollider) (+ VerticalVelocity (Transformation|GetVelocity)) false "None") ; Add the upward/downward movement to velocity if already moving
    (else
      (Physics|SetPhysicsLinearVelocity (Variables|Default|GetArrowHead) (+ VerticalVelocity (Transformation|GetVelocity) "100.000000,0.000000,0.000000") true "None") ; Force object to move when stopped,  may need a more practical solution
    ))
  (return (> ZVelocity 0.0)))