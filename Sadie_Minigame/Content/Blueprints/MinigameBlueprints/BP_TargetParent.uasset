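; Minigame target parent actor that groups target rings so they can be moved together to a random spot.
; It caches its start location on BeginPlay, and ChangeLocation picks a random horizontal point in a box around it.
; ParentRings disables ring collider physics, attaches the rings, calls ChangeLocation, then re-enables physics.
; An author note marks the move as broken because the rings unparent themselves, and debug prints remain.
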(event EventBeginPlay
  (Variables|Default|SetOriginalPos (Transformation|GetActorLocation)))

(fn ConstructionScript)

(fn ChangeLocation
  (Development|PrintString "New position hopefully")
  (Transformation|SetActorLocation (Math|Random|RandomPointinBoundingBox (Variables|Default|GetOriginalPos) "500.000000,500.000000,0.000000") false false) ; Does not work, target rings unparent themselves
)

(fn ParentRings
  (for _array_element (Variables|Default|GetTargetRings)
    (Physics|SetSimulatePhysics (Variables|/Game/Blueprints/MinigameBlueprints/BP_Target.BP_Target_C|GetCollider _array_element) false)
    (Transformation|AttachActorToActor _array_element self "None" "KeepRelative" "KeepRelative" "KeepRelative" false)
    (Development|PrintString (Utilities|String|ToString(Integer) (Utilities|Array|Length (Actor|GetAllChildActors true)))))
  (CallFunction|ChangeLocation)
  (for _array_element_2 (Variables|Default|GetTargetRings)
    (Physics|SetSimulatePhysics (Variables|/Game/Blueprints/MinigameBlueprints/BP_Target.BP_Target_C|GetCollider _array_element_2) true)))