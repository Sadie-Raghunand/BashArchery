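; BP_Target is a target ring for the archery minigame that scores a point when something hits it.
; On BeginPlay it finds the BP_TargetParent actor and sets its ring material to one of two options based on the Even flag.
; A hit adds a point for team 0 through the BP_ArcheryGamemode point counter, destroys the hitting actor, prints the score and tells the parent to change location.
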(event EventBeginPlay
  (CallFunction|InitValues))

(event Collision|EventHit
  (params (MyComp :type Primitive%20Component%20Object%20Reference) (Other :type Actor%20Object%20Reference) (OtherComp :type Primitive%20Component%20Object%20Reference) (bSelfMoved :type Boolean) (HitLocation :type Vector :default "0, 0, 0") (HitNormal :type Vector :default "0, 0, 0") (NormalImpulse :type Vector :default "0, 0, 0") (Hit :type Hit%20Result%20Structure%20%28by%20ref%29))
  (CallFunction|AddPointsonTargetHit Other))

(fn ConstructionScript)

(fn ChangeRingColor
  (if (Variables|Default|GetEven)
    (Rendering|Material|SetMaterial (Variables|Default|GetTargetRing) 0 "/AnimationSharing/AnimSharingRed.AnimSharingRed")
    (else
      (Rendering|Material|SetMaterial (Variables|Default|GetTargetRing) 0 "/Engine/MaterialTemplates/VertexAnimation/AdvancedFlag.AdvancedFlag"))))

(fn AddPointsonTargetHit
  (params (self2 :type Actor%20Object%20Reference))
  (bind _outactors (Actor|GetAllActorsOfClass "/Game/Blueprints/MinigameBlueprints/BP_ArcheryGamemode.BP_ArcheryGamemode_C"))
  (bind _output_get (Variables|Default|SetGameModeReference (Utilities|Array|Get(acopy) _outactors)))
  (Class|BasePointCounter|AddPoints (Class|MinigameBase|GetPointCounter _output_get) 0 1)
  (Actor|DestroyActor self2)
  (Development|PrintString (Utilities|String|ToString(Integer) (Class|BasePointCounter|GetPoints (Class|MinigameBase|GetPointCounter _output_get))))
  (Default|ChangeLocation (Variables|Default|GetTargetParent)))

(fn InitValues
  (bind _returnvalue (Actor|GetActorOfClass "/Game/Blueprints/MinigameBlueprints/BP_TargetParent.BP_TargetParent_C"))
  (Variables|Default|SetTargetParent _returnvalue)
  (CallFunction|ChangeRingColor))