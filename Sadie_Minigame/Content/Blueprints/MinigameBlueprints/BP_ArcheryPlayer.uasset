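; Player for a turn-based archery minigame driven by a flex controller, with keyboard movement for testing.
; Registers with the turn manager and places itself relative to its target.
; Rotation input yaws player and capture camera in fixed one-degree steps, clamped to ±45, ignoring input magnitude.
; Analog flex spawns a force-scaled arrow on the player's turn, decrementing ammo and rerolling wind; off-turn it adds to the wind value instead.
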(event Input|EnhancedActionEvents|EnhancedInputActionIA_Movement
  (params (ActionValue :type Vector%202D%20Structure) (ElapsedSeconds :type Float%20%28double-precision%29) (TriggeredSeconds :type Float%20%28double-precision%29) (InputAction :type Input%20Action%20Object%20Reference :default "/MinigameCore/Input/IA_Movement.IA_Movement"))
  (bind (_x _y) (Math|Vector2D|BreakVector2D ActionValue))
  (:Triggered
    (Development|PrintString (Utilities|String|ToString(Vector2d) ActionValue))
    (CallFunction|RotatePlayer (Math|Vector|MakeVector _x _y 0.0))))

(event Input|EnhancedActionEvents|EnhancedInputActionIA_AnalogFlex
  (params (ActionValue :type Float%20%28double-precision%29) (ElapsedSeconds :type Float%20%28double-precision%29) (TriggeredSeconds :type Float%20%28double-precision%29) (InputAction :type Input%20Action%20Object%20Reference :default "/LimbitlessBluetoothPlugin/InputActions/IA_AnalogFlex.IA_AnalogFlex"))
  (:Started
    (Utilities|IsValid InputAction
      (:Is%20Valid
        (Development|PrintString "Valid input")
        (Development|PrintString "SHOT ARROW")
        (CallFunction|ShootArrow (* ActionValue 1e+01)))
      (:Is%20Not%20Valid
        (Development|PrintString "Invalid input")))))

(event Input|EnhancedActionEvents|EnhancedInputActionIA_MediumFlex
  (params (ActionValue :type Boolean) (ElapsedSeconds :type Float%20%28double-precision%29) (TriggeredSeconds :type Float%20%28double-precision%29) (InputAction :type Input%20Action%20Object%20Reference :default "/LimbitlessBluetoothPlugin/InputActions/IA_MediumFlex.IA_MediumFlex"))
  ;[1 1 1] Test to see if input is different from analog flex
  (:Triggered
    (Development|PrintString "Medium flex detected" :!label _label))
  (:Started
    (goto _label)))

(event Input|EnhancedActionEvents|EnhancedInputActionIA_Button1
  (params (ActionValue :type Boolean) (ElapsedSeconds :type Float%20%28double-precision%29) (TriggeredSeconds :type Float%20%28double-precision%29) (InputAction :type Input%20Action%20Object%20Reference :default "/MinigameCore/Input/IA_Button1.IA_Button1")))

(event Input|EnhancedActionEvents|EnhancedInputActionIA_LightFlex
  (params (ActionValue :type Boolean) (ElapsedSeconds :type Float%20%28double-precision%29) (TriggeredSeconds :type Float%20%28double-precision%29) (InputAction :type Input%20Action%20Object%20Reference :default "/LimbitlessBluetoothPlugin/InputActions/IA_LightFlex.IA_LightFlex"))
  ;[1 1 1] Test to see if input is different from analog flex
  (:Triggered
    (Development|PrintString "Light flex" :!label _label))
  (:Started
    (goto _label)))

(event Input|EnhancedActionEvents|EnhancedInputActionIA_StrongFlex
  (params (ActionValue :type Boolean) (ElapsedSeconds :type Float%20%28double-precision%29) (TriggeredSeconds :type Float%20%28double-precision%29) (InputAction :type Input%20Action%20Object%20Reference :default "/LimbitlessBluetoothPlugin/InputActions/IA_StrongFlex.IA_StrongFlex"))
  ;[1 1 1] Test to see if input is different from analog flex
  (:Triggered
    (Development|PrintString "Strong flex" :!label _label))
  (:Started
    (goto _label)))

(event EventBeginPlay
  (CallFunction|InitValues))

(event EventTick
  (params (DeltaSeconds :type Float%20%28single-precision%29))
  (bind (_isrotating _controllerrotation) (CallFunction|ReadEulerRotation)) ; Get euler rotation of player
  (if _isrotating
    (CallFunction|RotatePlayer _controllerrotation)))

(fn ConstructionScript)

(fn ShootArrow
  (params (ForceOnArrow :type Float%20%28double-precision%29))
  (bind _camera (Variables|Default|GetCamera))
  (bind _scenecapture (Variables|/Script/MinigameCore.MinigameCapture|GetSceneCapture _camera))
  (bind _returnvalue (Transformation|GetWorldTransform _scenecapture))
  (bind (_location _rotation _scale) (Math|Transform|BreakTransform _returnvalue))
  (if (== (Variables|/Game/Blueprints/MinigameBlueprints/BP_TurnManager.BP_TurnManager_C|GetPlayerTurn (Variables|Default|GetTurnManager)) (Variables|Default|GetThisPlayerNum)) ; Prevent input if it is not this player's turn
    (bind _returnvalue_2 (Game|SpawnActorfromClass "/Game/Blueprints/MinigameBlueprints/BP_Arrow.BP_Arrow_C" (Math|Transform|MakeTransform (+ (Transformation|GetActorLocation _camera) "50.000000,0.000000,0.000000") _rotation _scale) "Undefined" 0 0)) ; Instantiate arrow, may switch to pooling?
    (bind _output_get (Variables|Default|SetArrow _returnvalue_2))
    (Variables|/Game/Blueprints/MinigameBlueprints/BP_Arrow.BP_Arrow_C|SetMultiplier _output_get ForceOnArrow)
    (Math|Integer|DecrementInt (Variables|Default|GetArrows)
      (:%20%20
        (CallFunction|RandomizeWindDirection)
        (if (<= (Variables|Default|GetArrows) 0) ; If arrows are out
          (Development|PrintString "Player is out of arrows, true")
          (Default|SetLastArrow (Variables|Default|GetArrow)))))
    (else
      (CallFunction|PlayersChangeWind ForceOnArrow) ; If it is not the player's turn, give them the ability to change the wind factor
    )))

(fn InitValues
  (bind _returnvalue (Actor|GetActorOfClass "/MinigameCore/BP_MinigameCapture.BP_MinigameCapture_C"))
  (Variables|Default|SetCamera _returnvalue)
  (bind _returnvalue_2 (Actor|GetActorOfClass "/Game/Blueprints/MinigameBlueprints/BP_TurnManager.BP_TurnManager_C"))
  (bind _output_get (Variables|Default|SetTurnManager _returnvalue_2))
  (Variables|Default|SetThisPlayerNum (Utilities|Array|Length (Variables|/Game/Blueprints/MinigameBlueprints/BP_TurnManager.BP_TurnManager_C|GetPlayers (Variables|Default|GetTurnManager)))) ; Set which turn this player has, 0-3
  (Utilities|Array|Add (Variables|/Game/Blueprints/MinigameBlueprints/BP_TurnManager.BP_TurnManager_C|GetPlayers _output_get) self)
  (Math|Integer|IncrementInt (Variables|/Game/Blueprints/MinigameBlueprints/BP_TurnManager.BP_TurnManager_C|GetTurnsTotal _output_get)
    (:%20%20
      (bind _foundwidgets (Widget|GetAllWidgetsOfClass "/Game/Blueprints/MinigameBlueprints/BP_WindUI.BP_WindUI_C" true))
      (Variables|Default|SetWindUI (Utilities|Array|Get(acopy) _foundwidgets))
      (CallFunction|RandomizeWindDirection)
      (CallFunction|SetPositionatBegining))))

(fn RotatePlayer
  (params (RotVal :type Vector :default "0.000000,0.000000,1.000000"))
  (bind _returnvalue (Math|Rotator|MakeRotator 0.0 0.0 1.0))
  (bind _inrange (CallFunction|ChangeTotalRotVal (.Yaw (Math|Rotator|BreakRotator _returnvalue))))
  (if _inrange ; Only if rotation is in range does the rotation occur, else do nothing
    (Transformation|AddRelativeRotation (Variables|Components|GetDefaultSceneRoot) _returnvalue false false)
    (Transformation|AddRelativeRotation (Variables|/Script/Engine.Actor|GetRootComponent (Variables|Default|GetCamera)) _returnvalue false false) ; Also move camera to match rotation
  ))

(fn RandomizeWindDirection
  (Variables|Default|SetWind (Math|Random|RandomFloatinRange -1e+01 1e+01))
  (Variables|/Script/UMG.TextBlock|SetText (Variables|/Game/Blueprints/MinigameBlueprints/BP_WindUI.BP_WindUI_C|GetTextBlock_33 (Variables|Default|GetWindUI)) (Utilities|Text|ToText(Float) (Variables|Default|GetWind) "HalfToEven")))

(fn PlayersChangeWind
  (params (WindAdditive :type Float%20%28double-precision%29))
  (bind _output_get (Variables|Default|SetWind (+ (Variables|Default|GetWind) WindAdditive)))
  (Variables|/Script/UMG.TextBlock|SetText (Variables|/Game/Blueprints/MinigameBlueprints/BP_WindUI.BP_WindUI_C|GetTextBlock_33 (Variables|Default|GetWindUI)) (Utilities|Text|ToText(Float) _output_get "HalfToEven"))
  (Development|PrintString (Utilities|String|ToString(Text) (Utilities|Text|ToText(Float) _output_get "HalfToEven")) true true "(R=0.997333,G=1.000000,B=0.953415,A=1.000000)"))

(fn ChangeTotalRotVal
  (params (ChangeVal :type Float%20%28double-precision%29))
  (if (Math|Float|InRange(Float) (+ ChangeVal (Variables|Default|GetTotalRotation)) -45.0 45.0) ; Check if in of range, do nothing if it isnt
    (Variables|Default|SetTotalRotation (+ ChangeVal (Variables|Default|GetTotalRotation))) ; Change variable value if it remains in range
    (return true) ; Return true, in range
    (else
      (return false) ; Return false, out of range
    )))

(fn SetPositionatBegining
  (Transformation|SetActorLocation (+ (Transformation|GetActorLocation (Utilities|Array|Get(acopy) (Variables|/Game/Blueprints/MinigameBlueprints/BP_TurnManager.BP_TurnManager_C|GetTargets (Variables|Default|GetTurnManager)) (Variables|Default|GetThisPlayerNum))) (Variables|Default|GetTargetOffset)) false false))

(fn ReadEulerRotation
  (bind _playerrotation (Variables|Components|GetPlayerRotation))
  (bind _returnvalue (Class|PlayerRotationComponent|GetDeltaRotation _playerrotation))
  (bind (_x _y _z) (Class|KismetMathLibrary|BreakQuat _returnvalue))
  (bind _returnvalue_2 (Math|Vector|MakeVector _x _y _z))
  (return (> (.X (Class|KismetMathLibrary|BreakVector3f _returnvalue_2)) 0.0) _returnvalue_2))

(fn PrintInputValueAssistFunct
  (bind _playerrotation (Variables|Components|GetPlayerRotation))
  (bind _returnvalue (Class|PlayerRotationComponent|GetRotationInputValue _playerrotation))
  (bind (_x _y _z) (Class|KismetMathLibrary|BreakQuat _returnvalue))
  (Development|PrintString (Utilities|String|ToString(Vector) (Math|Vector|MakeVector _x _y _z))))